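; BP_NPC is an NPC blueprint that can be grabbed and released by another object.
; CaptureUpdate stores the grabbed state and, while grabbed by a valid Grabber, records it, disables capsule collision and rotates the capsule to lie sideways.
; On release it clears the Grabber, restores query and physics collision and resets the capsule's world rotation to zero.
; The event graph holds no active logic.
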(fn `CaptureUpdate`
  (params (Grabbed :type Boolean) (Grabber :type "/Game/Blueprint/Character/BP_GenericCharacter Object Reference"))
  (bind _output_get (set `self.Grabbed` Grabbed))
  (if _output_get
    (`/Engine/EditorBlueprintResources/StandardMacros.IsValid` Grabber
      (:`Is Valid`
        (set `self.Grabber` Grabber)
        (`PrimitiveComponent.SetCollisionEnabled` (`self.CapsuleComponent`) "NoCollision")
        (`SceneComponent.K2_SetWorldRotation` (`self.CapsuleComponent`) (struct :`Yaw` 90.0 :`Roll` 90.0) false false)))
    (else
      (set `self.Grabber` null)
      (`PrimitiveComponent.SetCollisionEnabled` (`self.CapsuleComponent`) "QueryAndPhysics")
      (`SceneComponent.K2_SetWorldRotation` (`self.CapsuleComponent`) (struct) false false))))

(fn `UserConstructionScript`
  (`parent.UserConstructionScript`))