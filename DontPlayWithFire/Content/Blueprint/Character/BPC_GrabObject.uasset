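; Character component that lets the owner pick up, carry, drop and use NPCs, equipment and physics objects.
; Pickup input runs prioritized sphere overlaps (pawns, equipment, physics bodies), choosing the closest candidate and setting a pickup type.
; That type routes drop and shoot inputs to rescue release, equipment actions or an impulse throw; attack drives held melee weapons.
; Grabbed physics objects follow via PhysicsHandle and a looping timer that pauses when nothing is held.
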(event `Initialize Update Grab Item Position`
  ;[0 0.1529 1 0.5] Initialize Grab Item Position
  (bind _returnvalue (`KismetSystemLibrary.K2_SetTimerDelegate` (delegate `Update Grab Item Position`) 0.001 true true))
  (set `self.Timer Update Grab Item Position` _returnvalue))

(event `self.ReceiveBeginPlay`
  ;[0 0.1529 1 0.5] Begin Play
  (bind _asbp_generic_character (cast `/Game/Blueprint/Character/BP_GenericCharacter` (`self.GetOwner`)))
  (set `self.As BP Generic Character` _asbp_generic_character)
  (`self.Initialize Update Grab Item Position`)
  (bind _asplayer_controller (cast `PlayerController` (`Pawn.GetController` (`self.As BP Generic Character`))))
  (bind _returnvalue (pcsubsystem `EnhancedInputLocalPlayerSubsystem` _asplayer_controller))
  (`/Engine/EditorBlueprintResources/StandardMacros.IsValid` _returnvalue
    (:`Is Valid`
      (`EnhancedInputSubsystemInterface.AddMappingContext` _returnvalue "/Game/Input/IMC_PickupPhysicObject.IMC_PickupPhysicObject" 1 (struct)))))

(event `EnhancedInput|/Game/Input/Actions/IA_Pickup`
  (params (ActionValue :type Boolean) (ElapsedSeconds :type "Float (double-precision)") (TriggeredSeconds :type "Float (double-precision)") (InputAction :type "InputAction Object Reference" :default "/Game/Input/Actions/IA_Pickup.IA_Pickup"))
  ;[1 0 0.06535 0.5] PickUp Input
  (:`Started`
    (if (not (`self.Grabbing`))
      (`/Engine/EditorBlueprintResources/StandardMacros.IsValid` (`self.As BP Generic Character`)
        (:`Is Valid`
          (`self.PickUpHierarchy`))))))

(event `Update Grab Item Position`
  (bind _as_bp_generic_character (`self.As BP Generic Character`))
  ;[0 1 0.07739 0.5] Update Grab Item Position
  (if (`self.Grabbing`)
    (`PhysicsHandleComponent.SetTargetLocationAndRotation` (`/Game/Blueprint/Character/BP_GenericCharacter.PhysicsHandle` (`self.As BP Generic Character`)) (+ (`Actor.K2_GetActorLocation` _as_bp_generic_character) (* (`Actor.GetActorForwardVector` _as_bp_generic_character) 75.0)) (`Actor.K2_GetActorRotation` _as_bp_generic_character))
    (else
      (`KismetSystemLibrary.K2_PauseTimerHandle` (`self.Timer Update Grab Item Position`)))))

(event `EnhancedInput|/Game/Input/Actions/IA_DropItem`
  (params (ActionValue :type Boolean) (ElapsedSeconds :type "Float (double-precision)") (TriggeredSeconds :type "Float (double-precision)") (InputAction :type "InputAction Object Reference" :default "/Game/Input/Actions/IA_DropItem.IA_DropItem"))
  (bind _handequipement (`/Game/Blueprint/Character/BP_GenericCharacter.HandEquipement` (`self.As BP Generic Character`)))
  ;[1 0 0.06535 0.5] PickUp Input
  (:`Started`
    (if (`self.Grabbing`)
      (switch `/Game/Blueprint/Character/E_PickUpType` (`self.PickUpType`)
        (:`NewEnumerator0`
          (`/Game/Blueprint/Character/BP_PlayerFireMan.DropRescue` (`self.As BP Player Fire Man`) false)
          (set `self.Grabbing` false))
        (:`NewEnumerator1`
          (`/Engine/EditorBlueprintResources/StandardMacros.IsValid` _handequipement
            (:`Is Valid`
              (`/Game/Blueprint/Equipement/Master/BP_Master_Equipement.Drop Item` _handequipement)
              (set `self.Grabbing` false))))
        (:`NewEnumerator2`
          (`PhysicsHandleComponent.ReleaseComponent` (`/Game/Blueprint/Character/BP_GenericCharacter.PhysicsHandle` (`self.As BP Generic Character`)))
          (set `self.Pick Up Actor` null)
          (set `self.Grabbing` false))))))

(event `EnhancedInput|/Game/Input/Actions/IA_Attack`
  (params (ActionValue :type Boolean) (ElapsedSeconds :type "Float (double-precision)") (TriggeredSeconds :type "Float (double-precision)") (InputAction :type "InputAction Object Reference" :default "/Game/Input/Actions/IA_Attack.IA_Attack"))
  (:`Started`
    (bind _asbp_equipment_melee (cast `/Game/Blueprint/Equipement/Master/BP_Equipment_Melee` (`/Game/Blueprint/Character/BP_GenericCharacter.HandEquipement` (`self.As BP Generic Character`))))
    (`/Game/Blueprint/Equipement/Master/BP_Equipment_Melee.HittingStart` _asbp_equipment_melee))
  (:`Canceled`
    (bind _asbp_equipment_melee_2 (cast `/Game/Blueprint/Equipement/Master/BP_Equipment_Melee` (`/Game/Blueprint/Character/BP_GenericCharacter.HandEquipement` (`self.As BP Generic Character`)) :!label _label))
    (`/Game/Blueprint/Equipement/Master/BP_Equipment_Melee.HittingComplete` _asbp_equipment_melee_2))
  (:`Completed`
    (goto _label)))

(event `EnhancedInput|/Game/Input/Actions/IA_Shoot`
  (params (ActionValue :type Boolean) (ElapsedSeconds :type "Float (double-precision)") (TriggeredSeconds :type "Float (double-precision)") (InputAction :type "InputAction Object Reference" :default "/Game/Input/Actions/IA_Shoot.IA_Shoot"))
  (bind _as_bp_generic_character (`self.As BP Generic Character`))
  (bind _physicshandle (`/Game/Blueprint/Character/BP_GenericCharacter.PhysicsHandle` (`self.As BP Generic Character`)))
  (:`Triggered`
    (switch `/Game/Blueprint/Character/E_PickUpType` (`self.PickUpType`)
      (:`NewEnumerator1`
        (bind _asbp_equipement_range (cast `/Game/Blueprint/Equipement/Master/BP_Equipement_Range` (`/Game/Blueprint/Character/BP_GenericCharacter.HandEquipement` (`self.As BP Generic Character`))))
        (`/Game/Blueprint/Equipement/Master/BP_Equipement_Range.Shooting Triggered` _asbp_equipement_range))))
  (:`Started`
    (if (`self.Grabbing`)
      (switch `/Game/Blueprint/Character/E_PickUpType` (`self.PickUpType`)
        (:`NewEnumerator0`
          (`/Game/Blueprint/Character/BP_PlayerFireMan.DropRescue` (`self.As BP Player Fire Man`) true)
          (set `self.Grabbing` false))
        (:`NewEnumerator1`
          (switch `/Game/Blueprint/Character/E_PickUpType` (`self.PickUpType`)
            (:`NewEnumerator1`
              (bind _asbp_equipement_range_2 (cast `/Game/Blueprint/Equipement/Master/BP_Equipement_Range` (`/Game/Blueprint/Character/BP_GenericCharacter.HandEquipement` (`self.As BP Generic Character`))))
              (`/Game/Blueprint/Equipement/Master/BP_Equipement_Range.Shooting Started` _asbp_equipement_range_2))))
        (:`NewEnumerator2`
          (`/Game/Blueprint/Equipement/BPFL/BPFL_Raycast.PointingMiddleOfScreen` 3000.0 (`Character.Mesh` _as_bp_generic_character) "Bone1" "TraceTypeQuery1" (`|MakeArray` _as_bp_generic_character :!type "Actor Object Reference"))
          (bind _output_get (set `self.Physic component` (`PhysicsHandleComponent.GetGrabbedComponent` _physicshandle)))
          (`PhysicsHandleComponent.ReleaseComponent` _physicshandle)
          (`PhysicsObjectBlueprintLibrary.ApplyRadialImpulse` _output_get (`Actor.K2_GetActorLocation` (`self.As BP Generic Character`)) 250.0 1000.0 "RIF_Constant" false 0.0 true)
          (set `self.Pick Up Actor` null)
          (set `self.Grabbing` false)))))
  (:`Completed`
    (switch `/Game/Blueprint/Character/E_PickUpType` (`self.PickUpType`)
      (:`NewEnumerator1`
        (bind _asbp_equipement_range_3 (cast `/Game/Blueprint/Equipement/Master/BP_Equipement_Range` (`/Game/Blueprint/Character/BP_GenericCharacter.HandEquipement` (`self.As BP Generic Character`))))
        (`/Game/Blueprint/Equipement/Master/BP_Equipement_Range.Shooting Completed` _asbp_equipement_range_3)))))

(fn `PickUpEquipement`
  (params (Array :type "Array of Actor Object Reference") (Owner :type "Actor Object Reference"))
  (locals (L_Owner :type "Actor Object Reference") (L_ArrayActor :type "Actor Object Reference") (L_ArrayComponent :type "StaticMeshComponent Object Reference"))
  (bind _pickupequipementactor (`self.PickUpEquipementActor`))
  (set `local.L_Owner` Owner)
  (set `self.Closest Distance` (+ (`self.CasterSphereRadius`) 100.0))
  (for _array_element Array
    (bind _output_get (set `local.L_ArrayActor` _array_element))
    (bind _asbp_master_pick_up_items (cast `/Game/Blueprint/Equipement/Master/BP_Master_PickUpItems` _output_get))
    (bind _returnvalue (`Actor.GetDistanceTo` _asbp_master_pick_up_items (`local.L_Owner`)))
    (if (<= _returnvalue (`self.Closest Distance`))
      (set `self.Closest Distance` _returnvalue)
      (set `self.PickUpEquipementActor` _asbp_master_pick_up_items)))
  (`/Engine/EditorBlueprintResources/StandardMacros.IsValid` _pickupequipementactor
    (:`Is Valid`
      (`/Game/Blueprint/Equipement/Master/BP_Master_PickUpItems.PickupBehavior` _pickupequipementactor (`self.As BP Generic Character`))
      (set `self.Grabbing` true)
      (set `self.PickUpType` "NewEnumerator1"))))

(fn `PickUpHierarchy`
  (bind _pickupitemsequipementcandidate (`self.PickUpItemsEquipementCandidate`))
  ; Pawn PickUp
  (bind (_outactors _returnvalue) (`KismetSystemLibrary.SphereOverlapActors` (`self.CasterSpherePosition` 50.0) 200.0 (`|MakeArray` "ObjectTypeQuery3" :!type "EObjectTypeQuery Enum") null (`|MakeArray` (`self.GetOwner`))))
  (if _returnvalue
    (`self.PickUpPawn` _outactors (`self.GetOwner`))
    (else
      (`KismetArrayLibrary.Array_Clear` (`self.PickUpItemsEquipementCandidate`))
      ; Equipement PickUp
      (bind (_outactors_2 _returnvalue_2) (`KismetSystemLibrary.SphereOverlapActors` (`self.CasterSpherePosition` 50.0) (`self.CasterSphereRadius`) (`|MakeArray` "ObjectTypeQuery1" "ObjectTypeQuery2" :!type "EObjectTypeQuery Enum") null (`|MakeArray` (`self.GetOwner`))))
      (if _returnvalue_2
        (for _array_element _outactors_2
          (bind _asbp_master_pick_up_items (cast `/Game/Blueprint/Equipement/Master/BP_Master_PickUpItems` _array_element))
          (`KismetArrayLibrary.Array_Add` _pickupitemsequipementcandidate _asbp_master_pick_up_items))
        (`/Engine/EditorBlueprintResources/StandardMacros.IsValid` (`|GetArrayItem` _pickupitemsequipementcandidate)
          (:`Is Valid`
            (`self.PickUpEquipement` _pickupitemsequipementcandidate (`self.GetOwner`)))
          (:`Is Not Valid`
            ; Physic PickUp
            (bind (_outactors_3 _returnvalue_3) (`KismetSystemLibrary.SphereOverlapActors` (`self.CasterSpherePosition` 50.0) (`self.CasterSphereRadius`) (`|MakeArray` "ObjectTypeQuery4" "ObjectTypeQuery2" :!type "EObjectTypeQuery Enum") null (`|MakeArray` (`self.GetOwner`)) :!label _label))
            (if _returnvalue_3
              (`self.PickUpPhysicObject` _outactors_3 (`self.GetOwner`)))))
        (else
          (goto _label))))))

(fn `PickUpPawn`
  (params (Array :type "Array of Actor Object Reference") (Owner :type "Actor Object Reference"))
  (locals (L_Owner :type "Actor Object Reference") (L_ArrayActor :type "Actor Object Reference") (L_ArrayComponent :type "StaticMeshComponent Object Reference"))
  (bind _pickuppawnactor (`self.PickUpPawnActor`))
  (set `local.L_Owner` Owner)
  (set `self.Closest Distance` (+ (`self.CasterSphereRadius`) 100.0))
  (for _array_element Array
    (bind _output_get (set `local.L_ArrayActor` _array_element))
    (bind _asbp_npc (cast `/Game/Blueprint/Character/BP_NPC` _output_get))
    (bind _returnvalue (`Actor.GetDistanceTo` _asbp_npc (`local.L_Owner`)))
    (if (<= _returnvalue (`self.Closest Distance`))
      (set `self.Closest Distance` _returnvalue)
      (set `self.PickUpPawnActor` _asbp_npc)))
  (`/Engine/EditorBlueprintResources/StandardMacros.IsValid` _pickuppawnactor
    (:`Is Valid`
      (bind _asbp_player_fire_man (cast `/Game/Blueprint/Character/BP_PlayerFireMan` (`self.As BP Generic Character`)))
      (bind _output_get_2 (set `self.As BP Player Fire Man` _asbp_player_fire_man))
      (`/Game/Blueprint/Character/BP_PlayerFireMan.Rescueing` _output_get_2 _pickuppawnactor)
      (set `self.Grabbing` true)
      (set `self.PickUpType` "NewEnumerator0"))))

(fn `PickUpPhysicObject`
  (params (Array :type "Array of Actor Object Reference") (Owner :type "Actor Object Reference"))
  (locals (L_Owner :type "Actor Object Reference") (L_ArrayActor :type "Actor Object Reference") (L_ArrayComponent :type "StaticMeshComponent Object Reference"))
  (bind _pick_up_actor (`self.Pick Up Actor`))
  (set `local.L_Owner` Owner)
  (set `self.Closest Distance` (+ (`self.CasterSphereRadius`) 100.0))
  (for _array_element Array
    (bind _output_get (set `local.L_ArrayActor` _array_element))
    (`/Engine/EditorBlueprintResources/StandardMacros.IsValid` _output_get
      (:`Is Valid`
        (for _array_element_2 (`Actor.K2_GetComponentsByClass` _output_get "/Script/Engine.StaticMeshComponent")
          (bind _output_get_2 (set `local.L_ArrayComponent` _array_element_2))
          (`KismetSystemLibrary.PrintString` (`KismetSystemLibrary.GetDisplayName` (`local.L_ArrayActor`)) false true (`KismetMathLibrary.Conv_VectorToLinearColor` (`KismetMathLibrary.RandomUnitVector`)))
          (bind _returnvalue (`SceneComponent.K2_GetComponentLocation` _output_get_2))
          (`KismetSystemLibrary.LineTraceSingle` _returnvalue (+ _returnvalue (0.0 0.0 8000.0)) "TraceTypeQuery1" false (`|MakeArray` (`local.L_Owner`)))
          (bind _returnvalue_2 (`KismetMathLibrary.Vector_Distance` _returnvalue (`Actor.K2_GetActorLocation` (`local.L_Owner`))))
          (if (<= _returnvalue_2 (`self.Closest Distance`))
            (set `self.Closest Distance` _returnvalue_2)
            (set `self.Pick Up Actor` (`local.L_ArrayActor`)))))))
  (`/Engine/EditorBlueprintResources/StandardMacros.IsValid` _pick_up_actor
    (:`Is Valid`
      (for _array_element_3 (`Actor.K2_GetComponentsByClass` _pick_up_actor "/Script/Engine.StaticMeshComponent")
        (bind _output_get_3 (set `local.L_ArrayComponent` _array_element_3))
        (`/Engine/EditorBlueprintResources/StandardMacros.IsValid` _output_get_3
          (:`Is Valid`
            (`PhysicsHandleComponent.GrabComponentAtLocation` (`/Game/Blueprint/Character/BP_GenericCharacter.PhysicsHandle` (`self.As BP Generic Character`)) (`local.L_ArrayComponent`) "None" (`SceneComponent.K2_GetComponentLocation` _array_element_3))
            (set `self.Grabbing` true)
            (set `self.PickUpType` "NewEnumerator2")
            (`KismetSystemLibrary.K2_UnPauseTimerHandle` (`self.Timer Update Grab Item Position`))))))))