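; Character component that lets a BP_GenericCharacter grab and carry nearby physics objects while the pickup input is held.
; On BeginPlay it adds its own Enhanced Input mapping context.
; Pressing pickup sphere-overlaps physics bodies ahead, debug-prints them, and grabs the nearest one's static mesh with the character's PhysicsHandle.
; Tick keeps the handle target just in front of the character until release; a socket-attach alternative is left unconnected.
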(event `self.ReceiveBeginPlay`
  (bind _asbp_generic_character (cast `/Game/Blueprint/Character/BP_GenericCharacter` (`self.GetOwner`)))
  (set `self.As BP Generic Character` _asbp_generic_character)
  (bind _asplayer_controller (cast `PlayerController` (`Pawn.GetController` (`self.As BP Generic Character`))))
  (bind _returnvalue (pcsubsystem `EnhancedInputLocalPlayerSubsystem` _asplayer_controller))
  (`/Engine/EditorBlueprintResources/StandardMacros.IsValid` _returnvalue
    (:`Is Valid`
      (`EnhancedInputSubsystemInterface.AddMappingContext` _returnvalue "/Game/Input/IMC_PickupPhysicObject.IMC_PickupPhysicObject" 1 (struct)))))

(event `EnhancedInput|/Game/Input/Actions/IA_Pickup`
  (params (ActionValue :type Boolean) (ElapsedSeconds :type "Float (double-precision)") (TriggeredSeconds :type "Float (double-precision)") (InputAction :type "InputAction Object Reference" :default "/Game/Input/Actions/IA_Pickup.IA_Pickup"))
  (bind _returnvalue (`self.GetOwner`))
  (bind _as_bp_generic_character (`self.As BP Generic Character`))
  (bind _pick_up_actor (`self.Pick Up Actor`))
  (:`Started`
    (`/Engine/EditorBlueprintResources/StandardMacros.IsValid` _as_bp_generic_character
      (:`Is Valid`
        (set `self.Closest Distance` 300.0)
        (bind _outactors (`KismetSystemLibrary.SphereOverlapActors` (+ (`Actor.K2_GetActorLocation` _as_bp_generic_character) (* (`Actor.GetActorForwardVector` _as_bp_generic_character) 25.0)) 200.0 (`|MakeArray` "ObjectTypeQuery4" :!type "EObjectTypeQuery Enum") null (`|MakeArray` _returnvalue)))
        (for _array_element _outactors
          (`/Engine/EditorBlueprintResources/StandardMacros.IsValid` _array_element
            (:`Is Valid`
              (`KismetSystemLibrary.PrintString` (`KismetSystemLibrary.GetDisplayName` _array_element) true true (`KismetMathLibrary.Conv_VectorToLinearColor` (`KismetMathLibrary.RandomUnitVector`)))
              (bind _returnvalue_2 (`Actor.GetDistanceTo` _array_element _returnvalue))
              (if (<= _returnvalue_2 (`self.Closest Distance`))
                (set `self.Closest Distance` _returnvalue_2)
                (set `self.Pick Up Actor` _array_element)))))
        (`/Engine/EditorBlueprintResources/StandardMacros.IsValid` _pick_up_actor
          (:`Is Valid`
            (for _array_element_2 (`Actor.K2_GetComponentsByClass` _pick_up_actor "/Script/Engine.StaticMeshComponent")
              (`/Engine/EditorBlueprintResources/StandardMacros.IsValid` _array_element_2
                (:`Is Valid`
                  (`PhysicsHandleComponent.GrabComponentAtLocation` (`/Game/Blueprint/Character/BP_GenericCharacter.PhysicsHandle` (`self.As BP Generic Character`)) _array_element_2 "None" (`SceneComponent.K2_GetComponentLocation` _array_element_2))
                  (set `self.Grabbing` true))))
            (set `self.Pick Up Actor` null))))))
  (:`Completed`
    (if (`self.Grabbing`)
      (set `self.Grabbing` false)
      (`PhysicsHandleComponent.ReleaseComponent` (`/Game/Blueprint/Character/BP_GenericCharacter.PhysicsHandle` (`self.As BP Generic Character`))))))

(event `self.ReceiveTick`
  (params (DeltaSeconds :type "Float (single-precision)"))
  (bind _as_bp_generic_character (`self.As BP Generic Character`))
  (if (`self.Grabbing`)
    (`PhysicsHandleComponent.SetTargetLocation` (`/Game/Blueprint/Character/BP_GenericCharacter.PhysicsHandle` (`self.As BP Generic Character`)) (+ (`Actor.K2_GetActorLocation` _as_bp_generic_character) (* (`Actor.GetActorForwardVector` _as_bp_generic_character) 25.0)))))