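; Rescue game manager that plays background music and tallies insurance claims for damaged items.
; On BeginPlay it plays a random Music track on a new audio component, and each finish starts another.
; InsuranceClaim records unique damaged actors, then adds counts and costs by claim cause and item category.
; TotalItemCost increases in both CalculateClaimCategoryCost and CalculateTotalCost, so each claim counts twice there; UpdateRescue is an empty stub.
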(event `self.ReceiveBeginPlay`
  ;[0 0.1529 1 0.5] Begin Play
  (`self.Play audio`))

(event `Play audio`
  ;[1 0 0.06535 0.5] Play Audio
  (bind _returnvalue (`AddComponent|NODE_AddAudioComponent-0`))
  (add `AudioComponent.OnAudioFinished` _returnvalue (delegate `OnAudioFinished_Event`))
  (`AudioComponent.SetSound` _returnvalue (`KismetArrayLibrary.Array_Random` (`self.Music`)))
  (`AudioComponent.Play` _returnvalue 0.0)
  (bind _returnvalue_2 (message `AnimationDataModel.GetPlayLength` (`AudioComponent.Sound` _returnvalue)))
  (`KismetSystemLibrary.PrintString` (`KismetStringLibrary.Conv_DoubleToString` _returnvalue_2)))

(event `OnAudioFinished_Event`
  ;[1 0 0.06535 0.5] Play Audio
  (`self.Play audio`))

(event `InsuranceClaim`
  (params (DamagedActor :type "/Game/Blueprint/CombustibleObject/BP_Master_CombustibleObject Object Reference") (InsuranceClaim :type "/Game/Blueprint/Manager/Insurance/STR_InsuranceClaims Structure") (ClaimCategory :type "/Game/Blueprint/Manager/Insurance/E_ClaimCategory Enum" :default "NewEnumerator0"))
  ;[1 0 0.06535 0.5] Insurance Claim
  (`KismetArrayLibrary.Array_AddUnique` (`self.DamagedActors`) DamagedActor)
  (`self.CalculateClaimCategoryCost` InsuranceClaim ClaimCategory)
  (`self.CalculateItemCategoryCost` InsuranceClaim)
  (`self.CalculateTotalCost` InsuranceClaim))

(event `Update Rescue`
  (params (`Is Positive` :type Boolean))
  (if `Is Positive`
    _))

(fn `CalculateClaimCategoryCost`
  (params (`Insurance Claim` :type "/Game/Blueprint/Manager/Insurance/STR_InsuranceClaims Structure") (ClaimCategory :type "/Game/Blueprint/Manager/Insurance/E_ClaimCategory Enum" :default "NewEnumerator0"))
  (bind (_itemcategory _itemcost) (break `/Game/Blueprint/Manager/Insurance/STR_InsuranceClaims` `Insurance Claim`))
  (set `self.Total Item Cost` (+ (`self.Total Item Cost`) _itemcost))
  (switch `/Game/Blueprint/Manager/Insurance/E_ClaimCategory` ClaimCategory
    (:`NewEnumerator0`
      (`/Engine/EditorBlueprintResources/StandardMacros.IncrementInt` (`self.ItemClaimedForFire`)
        (:`  `
          (set `self.ItemCostForFire` (+ (`self.ItemCostForFire`) _itemcost)))))
    (:`NewEnumerator1`
      (`/Engine/EditorBlueprintResources/StandardMacros.IncrementInt` (`self.ItemClaimedForFlood`)
        (:`  `
          (set `self.ItemCostForFlood` (+ (`self.ItemCostForFlood`) _itemcost)))))
    (:`NewEnumerator2`
      (`/Engine/EditorBlueprintResources/StandardMacros.IncrementInt` (`self.ItemClaimedForDemolition`)
        (:`  `
          (set `self.ItemCostForDemolition` (+ (`self.ItemCostForDemolition`) _itemcost)))))
    (:`NewEnumerator3`
      (`/Engine/EditorBlueprintResources/StandardMacros.IncrementInt` (`self.ItemClaimedForTheft`)
        (:`  `
          (set `self.ItemCostForTheft` (+ (`self.ItemCostForTheft`) _itemcost)))))))

(fn `CalculateItemCategoryCost`
  (params (`Insurance Claim` :type "/Game/Blueprint/Manager/Insurance/STR_InsuranceClaims Structure"))
  (bind (_itemcategory _itemcost) (break `/Game/Blueprint/Manager/Insurance/STR_InsuranceClaims` `Insurance Claim`))
  (switch `/Game/Blueprint/Manager/Insurance/E_ItemCategory` _itemcategory
    (:`NewEnumerator0`
      (`/Engine/EditorBlueprintResources/StandardMacros.IncrementInt` (`self.ClaimedForStructuralItem`)
        (:`  `
          (set `self.CostForStructuralItem` (+ _itemcost (`self.CostForStructuralItem`))))))
    (:`NewEnumerator1`
      (`/Engine/EditorBlueprintResources/StandardMacros.IncrementInt` (`self.ClaimedForPersonalGoods`)
        (:`  `
          (set `self.CostForPersonalGoods` (+ _itemcost (`self.CostForPersonalGoods`))))))
    (:`NewEnumerator2`
      (`/Engine/EditorBlueprintResources/StandardMacros.IncrementInt` (`self.ClaimedForFurnitures`)
        (:`  `
          (set `self.CostForFurniture` (+ _itemcost (`self.CostForFurniture`))))))
    (:`NewEnumerator3`
      (`/Engine/EditorBlueprintResources/StandardMacros.IncrementInt` (`self.ClaimedForHomeAppliances`)
        (:`  `
          (set `self.CostForHomeAppliances` (+ _itemcost (`self.CostForHomeAppliances`))))))
    (:`NewEnumerator4`
      (`/Engine/EditorBlueprintResources/StandardMacros.IncrementInt` (`self.ClaimedForArts`)
        (:`  `
          (set `self.CostForArts` (+ _itemcost (`self.CostForArts`))))))
    (:`NewEnumerator6`
      (`/Engine/EditorBlueprintResources/StandardMacros.IncrementInt` (`self.ClaimedForOutdooring`)
        (:`  `
          (set `self.CostForOutdooring` (+ _itemcost (`self.CostForOutdooring`))))))
    (:`NewEnumerator7`
      (`/Engine/EditorBlueprintResources/StandardMacros.IncrementInt` (`self.ClaimedForVehicles`)
        (:`  `
          (set `self.CostForVehicles` (+ _itemcost (`self.CostForVehicles`))))))))

(fn `CalculateTotalCost`
  (params (`Insurance Claim` :type "/Game/Blueprint/Manager/Insurance/STR_InsuranceClaims Structure"))
  (set `self.Total Item Cost` (+ (`self.Total Item Cost`) (`.ItemCost_8_F5EA57B1496839F6C003E6B674DEB6C8` (break `/Game/Blueprint/Manager/Insurance/STR_InsuranceClaims` `Insurance Claim`)))))

(fn `UserConstructionScript`)