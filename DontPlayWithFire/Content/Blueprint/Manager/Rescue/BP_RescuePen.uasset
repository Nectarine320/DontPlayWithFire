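; BP_RescuePen is a rescue pen actor that reports what enters and leaves its collision box to a mission board.
; Overlap begin and end events pass the other actor to the mission board reference, if it is valid.
; The construction script resets actor scale, enforces a minimum RescuePenScale, then sizes and raises the collision box to match.
; It also moves four orange cones to the box corners and positions a text render.
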(event `self.PenCollisionbox.OnComponentBeginOverlap`
  (params (OverlappedComponent :type "PrimitiveComponent Object Reference") (OtherActor :type "Actor Object Reference") (OtherComp :type "PrimitiveComponent Object Reference") (OtherBodyIndex :type Integer) (bFromSweep :type Boolean) (SweepResult :type "HitResult Structure (by ref)"))
  (bind _as_bp_mission_board (`self.As BP Mission Board`))
  (`/Engine/EditorBlueprintResources/StandardMacros.IsValid` _as_bp_mission_board
    (:`Is Valid`
      (`/Game/Blueprint/Manager/Rescue/BP_MissionBoard.OverlapBeginBoardUpdate` _as_bp_mission_board OtherActor))))

(event `self.PenCollisionbox.OnComponentEndOverlap`
  (params (OverlappedComponent :type "PrimitiveComponent Object Reference") (OtherActor :type "Actor Object Reference") (OtherComp :type "PrimitiveComponent Object Reference") (OtherBodyIndex :type Integer))
  (bind _as_bp_mission_board (`self.As BP Mission Board`))
  (`/Engine/EditorBlueprintResources/StandardMacros.IsValid` _as_bp_mission_board
    (:`Is Valid`
      (`/Game/Blueprint/Manager/Rescue/BP_MissionBoard.OverlapEndBoardUpdate` _as_bp_mission_board OtherActor))))

(fn `UserConstructionScript`
  (bind (_rescuepenscale_x _rescuepenscale_y _rescuepenscale_z) (`KismetMathLibrary.BreakVector` (`self.RescuePenScale`)))
  (bind _rescuepenscale (`self.RescuePenScale`))
  (bind _x (.x (* (/ _rescuepenscale 2.0) 100.0)))
  (bind _y (.y (* (/ _rescuepenscale 2.0) 100.0)))
  (`self.SetActorScale3D` (1.0 1.0 1.0))
  (set `self.RescuePenScale` (`KismetMathLibrary.MakeVector` (`KismetMathLibrary.SelectFloat` 4.0 _rescuepenscale_x (<= _rescuepenscale_x 4.0)) (`KismetMathLibrary.SelectFloat` 4.0 _rescuepenscale_y (<= _rescuepenscale_y 4.0)) (`KismetMathLibrary.SelectFloat` 3.0 _rescuepenscale_z (<= _rescuepenscale_z 3.0))))
  (`SceneComponent.SetRelativeScale3D` (`self.PenCollisionbox`) _rescuepenscale)
  (`SceneComponent.K2_SetRelativeLocation` (`self.PenCollisionbox`) (`KismetMathLibrary.MakeVector` 0.0 0.0 (.z (* (/ _rescuepenscale 2.0) 100.0))) false false)
  (`SceneComponent.K2_SetRelativeLocation` (`self.OrangeCone_01`) (`KismetMathLibrary.MakeVector` _x _y) false false)
  (`SceneComponent.K2_SetRelativeLocation` (`self.OrangeCone_02`) (`KismetMathLibrary.MakeVector` _x (* -1.0 _y)) false false)
  (`SceneComponent.K2_SetRelativeLocation` (`self.OrangeCone_03`) (`KismetMathLibrary.MakeVector` (* -1.0 _x) _y) false false)
  (`SceneComponent.K2_SetRelativeLocation` (`self.OrangeCone_04`) (`KismetMathLibrary.MakeVector` (* -1.0 _x) (* -1.0 _y)) false false)
  (`SceneComponent.K2_SetRelativeLocationAndRotation` (`self.TextRender`) (0.0 0.0 12.5) (struct :`Pitch` 90.0) false false))