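; BPC_Destructible is a component that breaks its owning object in stages each time it receives a hit, with a hammering or wall-specific sound.
; Each hit advances a clamped state index and swaps meshes, either one static mesh or three wall meshes on a BP_Master_CombustibleObject flagged as a wall.
; State changes trigger the owner's insurance claim, and the last state alters collision, while an empty mesh slot destroys the actor.
; Non-destructible objects get an impulse instead.
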(event `self.ReceiveBeginPlay`
  (bind (_asbp_master_combustible_object _bsuccess) (cast `/Game/Blueprint/CombustibleObject/BP_Master_CombustibleObject` (`self.GetOwner`) :!pure true))
  (if _bsuccess
    (set `self.As BP Master Combustible Object` _asbp_master_combustible_object)))

(event `Hit recieved`
  (params (`Impact Location` :type "Vector Structure") (`Impact Normal` :type "Vector Structure"))
  (bind _as_bp_master_combustible_object (`self.As BP Master Combustible Object`))
  (`/Engine/EditorBlueprintResources/StandardMacros.IsValid` _as_bp_master_combustible_object
    (:`Is Valid`
      (if (`/Game/Blueprint/CombustibleObject/BP_Master_CombustibleObject.IsWall` _as_bp_master_combustible_object)
        (`self.WallMeshHit` `Impact Normal`)
        (else
          (`self.SingleMeshHit` `Impact Normal` :!label _label))))
    (:`Is Not Valid`
      (goto _label))))

(fn `Claim Insurance`
  (bind _as_bp_master_combustible_object (`self.As BP Master Combustible Object`))
  (`/Engine/EditorBlueprintResources/StandardMacros.IsValid` _as_bp_master_combustible_object
    (:`Is Valid`
      (`/Game/Blueprint/CombustibleObject/BP_Master_CombustibleObject.ClaimInsurance` _as_bp_master_combustible_object "NewEnumerator2"))))

(fn `SingleMeshHit`
  (params (ImpactNormal :type "Vector Structure"))
  (bind _staticmeshstate (`self.StaticMeshState`))
  (bind _current_state (`self.Current State`))
  (bind _returnvalue (`Actor.GetComponentByClass` (`self.GetOwner`) "/Script/Engine.StaticMeshComponent"))
  (bind _returnvalue_2 (`Actor.GetComponentByClass` (`self.GetOwner`) "/Script/Engine.StaticMeshComponent"))
  (bind _output (`|GetArrayItem` _staticmeshstate (`self.Current State`)))
  (`GameplayStatics.PlaySound2D` "/Game/Audio/NotLegitAudio/SFX/Hammering/SFX_Hammering.SFX_Hammering" 1.0 1.0 0.0 null null)
  (if (`self.CanBeDestroyed`)
    (bind _result (`/Engine/EditorBlueprintResources/StandardMacros.IncrementInt` _current_state)
      (:`  `
        (set `self.Current State` (`KismetMathLibrary.Clamp` _result 0 (`KismetArrayLibrary.Array_LastIndex` (`self.StaticMeshState`))))
        (`/Engine/EditorBlueprintResources/StandardMacros.IsValid` _returnvalue_2
          (:`Is Valid`
            (`/Engine/EditorBlueprintResources/StandardMacros.IsValid` _output
              (:`Is Valid`
                (`StaticMeshComponent.SetStaticMesh` _returnvalue_2 _output)
                (`self.Claim Insurance` :!label _label)
                (if (== (`KismetArrayLibrary.Array_LastIndex` _staticmeshstate) _current_state)
                  (`PrimitiveComponent.SetCollisionEnabled` _returnvalue_2 (`self.Last Index Collision`))))
              (:`Is Not Valid`
                (`|ExecutionSequence`
                  (:`then_0`
                    (goto _label))
                  (:`then_1`
                    (`Actor.K2_DestroyActor` (`self.GetOwner`))))))))))
    (else
      (`/Engine/EditorBlueprintResources/StandardMacros.IsValid` _returnvalue
        (:`Is Valid`
          (`PrimitiveComponent.AddImpulse` _returnvalue (* ImpactNormal 500.0) "None" true))))))

(fn `WallMeshHit`
  (params (ImpactNormal :type "Vector Structure"))
  (bind _as_bp_master_combustible_object (`self.As BP Master Combustible Object`))
  (bind _current_state (`self.Current State`))
  (bind _returnvalue (`Actor.GetComponentByClass` (`self.GetOwner`) "/Script/Engine.StaticMeshComponent"))
  (bind (_wall01 _inbetween _wall02) (break `/Game/Blueprint/CombustibleObject/STR_Wall` (`|GetArrayItem` (`.DestructibleState_3_D65A5BFC4FAC6C6B845734A314E4CD8D` (break `/Game/Blueprint/CombustibleObject/STR_DestructibleWall` (`self.DestructibleWallState`))) (`self.Current State`))))
  (`GameplayStatics.PlaySound2D` (`.HitSFX_19_EFF4C5B74A5BB19575709D8E92DDF7A1` (break `/Game/Blueprint/CombustibleObject/STR_DestructibleWall` (`self.DestructibleWallState`))) 1.0 1.0 0.0 null null)
  (if (`self.CanBeDestroyed`)
    (bind _result (`/Engine/EditorBlueprintResources/StandardMacros.IncrementInt` _current_state)
      (:`  `
        (set `self.Current State` (`KismetMathLibrary.Clamp` _result 0 (`KismetArrayLibrary.Array_LastIndex` (`.DestructibleState_3_D65A5BFC4FAC6C6B845734A314E4CD8D` (break `/Game/Blueprint/CombustibleObject/STR_DestructibleWall` (`self.DestructibleWallState`))))))
        (`StaticMeshComponent.SetStaticMesh` (`/Game/Blueprint/CombustibleObject/BP_Master_CombustibleObject.SM_Wall_01` (`self.As BP Master Combustible Object`)) _wall01)
        (`StaticMeshComponent.SetStaticMesh` (`/Game/Blueprint/CombustibleObject/BP_Master_CombustibleObject.SM_CombustibleObject` _as_bp_master_combustible_object) _inbetween)
        (`StaticMeshComponent.SetStaticMesh` (`/Game/Blueprint/CombustibleObject/BP_Master_CombustibleObject.SM_Wall_02` _as_bp_master_combustible_object) _wall02)
        (`self.Claim Insurance`)
        (if (== (`KismetArrayLibrary.Array_LastIndex` (`.DestructibleState_3_D65A5BFC4FAC6C6B845734A314E4CD8D` (break `/Game/Blueprint/CombustibleObject/STR_DestructibleWall` (`self.DestructibleWallState`)))) _current_state)
          (`PrimitiveComponent.SetCollisionEnabled` (`/Game/Blueprint/CombustibleObject/BP_Master_CombustibleObject.SM_Wall_01` (`self.As BP Master Combustible Object`)) (`self.Last Index Collision`))
          (`PrimitiveComponent.SetCollisionEnabled` (`/Game/Blueprint/CombustibleObject/BP_Master_CombustibleObject.SM_CombustibleObject` (`self.As BP Master Combustible Object`)) (`self.Last Index Collision`))
          (`PrimitiveComponent.SetCollisionEnabled` (`/Game/Blueprint/CombustibleObject/BP_Master_CombustibleObject.SM_Wall_02` (`self.As BP Master Combustible Object`)) (`self.Last Index Collision`)))))
    (else
      (`/Engine/EditorBlueprintResources/StandardMacros.IsValid` _returnvalue
        (:`Is Valid`
          (`PrimitiveComponent.AddImpulse` _returnvalue (* ImpactNormal 500.0) "None" true))))))