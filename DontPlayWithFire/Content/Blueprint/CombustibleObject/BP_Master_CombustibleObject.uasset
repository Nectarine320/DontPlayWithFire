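; Master combustible object that ignites, spreads fire, burns out or can be doused, filing an insurance claim with BP_RescueGM once burning.
; Timelines drive ignition, burning and burnout through a dynamic material, Niagara effects and status text.
; Once burning, a size-preset collision box ignites overlapping combustibles, while dowsing volumes reverse the ignition timeline.
; Pressurized objects explode, launching characters and adding impulse and ignition to nearby combustibles.
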(event `self.ReceiveBeginPlay`
  ;[0 0.4851 1 0.5] Begin Play
  (`PrimitiveComponent.SetCollisionEnabled` (`self.Progation Collision Box`) "NoCollision")
  (`MaterialInstanceDynamic.SetScalarParameterValue` (`self.BurningShader`) "Range" (`self.FadeRange`))
  (`self.SetPropagationSize` false)
  (bind _asbp_rescue_gm (cast `/Game/Blueprint/Manager/BP_RescueGM` (`GameplayStatics.GetGameMode`))
    (:`then`
      (set `self.As BP Rescue GM` _asbp_rescue_gm))
    (:`CastFailed`
      _))
  (if (`self.IgnitionAtStart`)
    (`self.Ignite`)))

(event `IgniteAnimation`
  ;[1.5 1.093 0 0.5] Ignition Animation
  (`ActorComponent.Activate` (`self.NS_IgniteSmoke`) false)
  (`self.IgnitionLifetime`)
  (`self.IgniteTextAnim`)
  (bind (_direction _ignitionalpha) (`Timeline|IgnitionTimeline` :`NewTime` (`self.IgnitionValue`) :!label _label)
    (:`Update`
      (set `self.IgnitionValue` _ignitionalpha)
      (`MaterialInstanceDynamic.SetScalarParameterValue` (`self.BurningShader`) "FireVisibility" (`KismetMathLibrary.Lerp` 0.0 0.5 _ignitionalpha)))
    (:`Finished`
      (switch `ETimelineDirection` _direction
        (:`Forward`
          (`self.IgnitionComplete`))
        (:`Backward`
          (`self.IgnitionReverted`))))))

(event `self.SM_CombustibleObject.OnComponentBeginOverlap`
  (params (OverlappedComponent :type "PrimitiveComponent Object Reference") (OtherActor :type "Actor Object Reference") (OtherComp :type "PrimitiveComponent Object Reference") (OtherBodyIndex :type Integer) (bFromSweep :type Boolean) (SweepResult :type "HitResult Structure (by ref)"))
  ;[1 0 0.06535 0.5] 💦- Dowsing Logic
  (bind _asbp_master_dowsing_volume (cast `/Game/Blueprint/DowsingVolumes/BP_Master_DowsingVolume` OtherActor))
  (`KismetArrayLibrary.Array_Add` (`self.DowsingVolumes`) _asbp_master_dowsing_volume)
  (`self.Initiate DowsingProtocol`))

(event `CancelledIgniteAnimation`
  ;[1.5 1.093 0 0.5] Ignition Animation
  (`self.CancelTextAnim`)
  (goto _label :!via `Stop`))

(event `self.SM_CombustibleObject.OnComponentEndOverlap`
  (params (OverlappedComponent :type "PrimitiveComponent Object Reference") (OtherActor :type "Actor Object Reference") (OtherComp :type "PrimitiveComponent Object Reference") (OtherBodyIndex :type Integer))
  ;[1 0 0.06535 0.5] 💦- Dowsing Logic
  (bind _asbp_master_dowsing_volume (cast `/Game/Blueprint/DowsingVolumes/BP_Master_DowsingVolume` OtherActor))
  (`KismetArrayLibrary.Array_RemoveItem` (`self.DowsingVolumes`) _asbp_master_dowsing_volume)
  (`self.Stop Dowsing Protocol`))

(event `ReverseIgniteAnimation`
  ;[1.5 1.093 0 0.5] Ignition Animation
  (`self.ExtinctionTextAnim`)
  (`self.ExtinctionLifetime`)
  (`SceneComponent.SetVisibility` (`self.WBP_Combustion`) true false)
  (goto _label :!via `Reverse`))

(event `Initiate DowsingProtocol`
  ;[1 0 0.06535 0.5] 💦- Dowsing Logic
  (`self.DowsingProtocol`))

(event `Stop Dowsing Protocol`
  ;[1 0 0.06535 0.5] 💦- Dowsing Logic
  (`/Engine/EditorBlueprintResources/StandardMacros.IsValid` (`|GetArrayItem` (`self.DowsingVolumes`))
    (:`Is Not Valid`
      (set `self.Dowsed` false)
      (`self.Cancelled Ignition`))))

(event `BurningAnimation`
  ;[1.5 1.093 0 0.5] Burning Animation Loop
  (`self.BurningTextAnim`)
  (bind (_direction _burningshaderlerp) (`Timeline|BurningVisualTimeline` :!label _label_2)
    (:`Update`
      (bind _returnvalue (`KismetMathLibrary.LinearColorLerp` (struct :`R` 0.75 :`G` 0.423534 :`A` 1.0) (struct :`R` 0.026042 :`G` 0.014706 :`A` 2.0) _burningshaderlerp))
      (set `self.CurrentBurningColor` _returnvalue)
      (`MaterialInstanceDynamic.SetVectorParameterValue` (`self.BurningShader`) "FireColor" _returnvalue))))

(event `self.Widget_CombustionSphere.OnComponentBeginOverlap`
  (params (OverlappedComponent :type "PrimitiveComponent Object Reference") (OtherActor :type "Actor Object Reference") (OtherComp :type "PrimitiveComponent Object Reference") (OtherBodyIndex :type Integer) (bFromSweep :type Boolean) (SweepResult :type "HitResult Structure (by ref)"))
  ;[1 0 0.06535 0.5] Widget Display Logic
  (if (== OtherActor (`GameplayStatics.GetPlayerCharacter` 0))
    (`SceneComponent.SetHiddenInGame` (`self.WBP_Combustion`) false false)))

(event `StopBurningVisualAnimation`
  ;[1.5 1.093 0 0.5] Burning Animation Loop
  (goto _label_2 :!via `Stop`))

(event `Extinguish Succeed`
  ;[1.5 1.093 0 0.5] Burning Animation Loop
  (`|ExecutionSequence`
    (:`then_0`
      (goto _label_2 :!via `Stop`))
    (:`then_1`
      (bind _direction (`Timeline|BurningLifeTimeline` :!via `Stop` :!label _label_3)
        (:`Finished`
          (switch `ETimelineDirection` _direction
            (:`Forward`
              (`self.StopBurningVisualAnimation`)
              (`self.Burn Out`))))))))

(event `self.Widget_CombustionSphere.OnComponentEndOverlap`
  (params (OverlappedComponent :type "PrimitiveComponent Object Reference") (OtherActor :type "Actor Object Reference") (OtherComp :type "PrimitiveComponent Object Reference") (OtherBodyIndex :type Integer))
  ;[1 0 0.06535 0.5] Widget Display Logic
  (if (== OtherActor (`GameplayStatics.GetPlayerCharacter` 0))
    (`SceneComponent.SetHiddenInGame` (`self.WBP_Combustion`) true false)))

(event `BurningDuration`
  ;[1.5 1.093 0 0.5] Burning Animation Loop
  (goto _label_3))

(event `Ignite`
  ;[1 0 0.06535 0.5] Ignition
  (if (not (or (`self.Burning`) (`self.BurntOut`)))
    (`self.IgnitionMultiplier`)
    (`self.IgniteAnimation`)))

(event `self.Progation Collision Box.OnComponentBeginOverlap`
  (params (OverlappedComponent :type "PrimitiveComponent Object Reference") (OtherActor :type "Actor Object Reference") (OtherComp :type "PrimitiveComponent Object Reference") (OtherBodyIndex :type Integer) (bFromSweep :type Boolean) (SweepResult :type "HitResult Structure (by ref)"))
  ;[1 0 0.06535 0.5] 🔥 - Propagation Logic
  (if (not (`self.Dowsed`))
    (bind _asbp_master_combustible_object (cast `/Game/Blueprint/CombustibleObject/BP_Master_CombustibleObject` OtherActor))
    (if (== OtherComp (`/Game/Blueprint/CombustibleObject/BP_Master_CombustibleObject.SM_CombustibleObject` _asbp_master_combustible_object))
      (`KismetArrayLibrary.Array_Add` (`/Game/Blueprint/CombustibleObject/BP_Master_CombustibleObject.CombustibleVolumes` _asbp_master_combustible_object) _asbp_master_combustible_object)
      (`self.Ignite` _asbp_master_combustible_object))))

(event `Cancelled Ignition`
  ;[1 0 0.06535 0.5] Ignition
  (if (not (`self.Burning`))
    (`self.CancelledIgniteAnimation`)))

(event `Burn Out`
  ;[1.5 1.093 0 0.5] Burnout Animation
  (set `self.BurntOut` true)
  (`self.BurntOutVFX`)
  (`self.CancelTextAnim`)
  (`self.Disable Propagation`)
  (if (`self.TurnIntoAshes`)
    (`ActorComponent.Deactivate` (`self.BPC_Destructible`))
    (`StaticMeshComponent.SetStaticMesh` (`self.SM_CombustibleObject`) (`self.BurntoutAshesMesh`))
    (else
      (bind (_direction _burnoutlerp) (`Timeline|BurnoutTimeline` :!via `PlayFromStart`)
        (:`Update`
          (`MaterialInstanceDynamic.SetVectorParameterValue` (`self.BurningShader`) "FireColor" (`KismetMathLibrary.LinearColorLerp` (`self.CurrentBurningColor`) (struct :`A` 2.0) _burnoutlerp)))))))

(event `self.Progation Collision Box.OnComponentEndOverlap`
  (params (OverlappedComponent :type "PrimitiveComponent Object Reference") (OtherActor :type "Actor Object Reference") (OtherComp :type "PrimitiveComponent Object Reference") (OtherBodyIndex :type Integer))
  ;[1 0 0.06535 0.5] 🔥 - Propagation Logic
  (if (not (`self.Dowsed`))
    (bind _asbp_master_combustible_object (cast `/Game/Blueprint/CombustibleObject/BP_Master_CombustibleObject` OtherActor))
    (if (== OtherComp (`/Game/Blueprint/CombustibleObject/BP_Master_CombustibleObject.SM_CombustibleObject` _asbp_master_combustible_object))
      (bind _combustiblevolumes (`/Game/Blueprint/CombustibleObject/BP_Master_CombustibleObject.CombustibleVolumes` _asbp_master_combustible_object))
      (`KismetArrayLibrary.Array_RemoveItem` _combustiblevolumes _asbp_master_combustible_object)
      (`/Engine/EditorBlueprintResources/StandardMacros.IsValid` (`|GetArrayItem` _combustiblevolumes)
        (:`Is Valid`
          (`self.Cancelled Ignition` _asbp_master_combustible_object))))))

(event `Reverse Ignition`
  ;[1 0 0.06535 0.5] Ignition
  (if (`self.Burning`)
    (set `self.Burning` false))
  (`self.ReverseIgniteAnimation`))

(event `Enable Propagation`
  ;[1 0 0.06535 0.5] 🔥 - Propagation Logic
  (`PrimitiveComponent.SetCollisionEnabled` (`self.Progation Collision Box`) "QueryOnly"))

(event `Disable Propagation`
  ;[1 0 0.06535 0.5] 🔥 - Propagation Logic
  (`PrimitiveComponent.SetCollisionEnabled` (`self.Progation Collision Box`) "NoCollision"))

(event `ExtinctionTextAnim`
  ;[1.5 1.093 0 0.5] Text Update Anim
  (`self.Stop Text Animation` true false)
  (`Timeline|ExtinctionTextAnimation` :!label _label_4
    (:`NewTrack_0`
      (set `self.TextStatus` "Extiguishing"))
    (:`NewTrack_1`
      (set `self.TextStatus` "Extiguishing."))
    (:`NewTrack_2`
      (set `self.TextStatus` "Extiguishing.."))
    (:`NewTrack_3`
      (set `self.TextStatus` "Extiguishing..."))))

(event `Stop Extinction Text Animation`
  ;[1.5 1.093 0 0.5] Text Update Anim
  (goto _label_4 :!via `Stop`))

(event `IgniteTextAnim`
  ;[1.5 1.093 0 0.5] Text Update Anim
  (`self.Stop Text Animation` false))

(event `Stop Ignite Text Animation`
  ;[1.5 1.093 0 0.5] Text Update Anim
  (`Timeline|IgniteTextAnimation` :!via `Stop`
    (:`NewTrack_0`
      (set `self.TextStatus` "Igniting"))
    (:`NewTrack_1`
      (set `self.TextStatus` "Igniting."))
    (:`NewTrack_2`
      (set `self.TextStatus` "Igniting.."))
    (:`NewTrack_3`
      (set `self.TextStatus` "Igniting..."))))

(event `CancelTextAnim`
  ;[1.5 1.093 0 0.5] Text Update Anim
  (`self.Stop Text Animation` true))

(event `BurningTextAnim`
  ;[1.5 1.093 0 0.5] Text Update Anim
  (`self.Stop Text Animation` true true false))

(event `Stop Burning Text Animation`
  ;[1.5 1.093 0 0.5] Text Update Anim
  (`Timeline|BurningTextAnimation` :!via `Stop`
    (:`NewTrack_0`
      _)
    (:`NewTrack_1`
      _)
    (:`NewTrack_2`
      _)
    (:`NewTrack_3`
      _))
  (`/Engine/EditorBlueprintResources/StandardMacros.FlipFlop`))

(fn `AwakePhysics`
  (if (`PrimitiveComponent.IsAnyRigidBodyAwake` (`self.SM_CombustibleObject`))
    _))

(fn `BlastCharacter`
  (params (Character :type "Character Object Reference") (ExplosionLocation :type "Vector Structure") (BlastRadius :type "Float (single-precision)"))
  (bind _returnvalue (`self.K2_GetActorLocation` Character))
  (bind _returnvalue_2 (`KismetMathLibrary.Vector_Distance` _returnvalue ExplosionLocation))
  (if (<= _returnvalue_2 BlastRadius)
    (`Character.LaunchCharacter` Character (+ (* (`KismetMathLibrary.GetDirectionUnitVector` ExplosionLocation _returnvalue) (* (/ BlastRadius _returnvalue_2) (* (`self.ExplosionStrength`) 0.1))) (0.0 0.0 250.0)) false false)))

(fn `BlastObject`
  (params (CombustibleObject :type "/Game/Blueprint/CombustibleObject/BP_Master_CombustibleObject Object Reference") (ExplosionLocation :type "Vector Structure") (BlastRadius :type "Float (single-precision)"))
  (bind _explosiondamage (`self.ExplosionDamage`))
  (if (not (== CombustibleObject self))
    (`PhysicsObjectBlueprintLibrary.ApplyRadialImpulse` (`/Game/Blueprint/CombustibleObject/BP_Master_CombustibleObject.SM_CombustibleObject` CombustibleObject) ExplosionLocation BlastRadius (`self.ExplosionStrength`) "RIF_Linear" false 0.0 true)
    (bind _output_get (set `/Game/Blueprint/CombustibleObject/BP_Master_CombustibleObject.IgnitionValue` (`KismetMathLibrary.FClamp` (+ (`/Game/Blueprint/CombustibleObject/BP_Master_CombustibleObject.IgnitionValue` CombustibleObject) _explosiondamage (* _explosiondamage (/ BlastRadius (`KismetMathLibrary.Vector_Distance` ExplosionLocation (`self.K2_GetActorLocation` CombustibleObject)))))) CombustibleObject))
    (if (>= _output_get 1.0)
      (`self.IgnitionComplete` CombustibleObject))))

(fn `BurntOutVFX`
  (`ActorComponent.Deactivate` (`self.NS_BurningSmoke`))
  (`ActorComponent.Deactivate` (`self.NS_Fire`))
  (`ActorComponent.Activate` (`self.NS_BurntOutSmoke`) false))

(fn `ClaimInsurance`
  (params (ClaimCategory :type "/Game/Blueprint/Manager/Insurance/E_ClaimCategory Enum" :default "NewEnumerator0"))
  (if (not (`self.IsFileClaimed`))
    (set `self.IsFileClaimed` true)
    (`/Game/Blueprint/Manager/BP_RescueGM.InsuranceClaim` (`self.As BP Rescue GM`) self (`/Game/Blueprint/Manager/Insurance/PDA_InsuranceClaim.InsuranceClaim` (`self.Insurance Claim`)) ClaimCategory)))

(fn `DowsingProtocol`
  (set `self.Dowsed` true)
  (`self.Reverse Ignition`))

(fn `Explosion`
  (bind _exploded_mesh (`self.Exploded Mesh`))
  (bind _blastradiuscapsule (`self.BlastRadiusCapsule`))
  (bind _returnvalue (`SceneComponent.K2_GetComponentLocation` (`self.Progation Collision Box`)))
  (set `self.HasExploded` true)
  (`ActorComponent.Activate` (`self.CPS_Explosion`) false)
  (`/Engine/EditorBlueprintResources/StandardMacros.IsValid` _exploded_mesh
    (:`Is Valid`
      (`StaticMeshComponent.SetStaticMesh` (`self.SM_CombustibleObject`) _exploded_mesh))
    (:`Is Not Valid`
      _))
  (bind _outactors (`KismetSystemLibrary.SphereOverlapActors` _returnvalue _blastradiuscapsule (`self.Object Types`) null (`|MakeArray` self :!type "Actor Object Reference")))
  (for _array_element _outactors
    (bind _asbp_master_combustible_object (cast `/Game/Blueprint/CombustibleObject/BP_Master_CombustibleObject` _array_element)
      (:`then`
        (`self.BlastObject` _asbp_master_combustible_object _returnvalue _blastradiuscapsule))
      (:`CastFailed`
        (bind _aspersonnage (cast `Character` _array_element))
        (`self.BlastCharacter` _aspersonnage _returnvalue _blastradiuscapsule)))))

(fn `ExtinctionLifetime`
  (bind _ignitiontimeline (`self.IgnitionTimeline`))
  (`TimelineComponent.SetPlayRate` _ignitiontimeline (/ (`TimelineComponent.GetTimelineLength` _ignitiontimeline) (`self.DowsingTimeRequitement`))))

(fn `IgnitionComplete`
  (if (not (`self.HasExploded`))
    (set `self.Burning` true)
    (`self.Enable Propagation`)
    (`self.BurningAnimation`)
    (`self.ClaimInsurance` "NewEnumerator0")
    (`ActorComponent.Activate` (`self.NS_BurningSmoke`) false)
    (`ActorComponent.Activate` (`self.NS_Fire`) false)
    (`ActorComponent.Deactivate` (`self.NS_IgniteSmoke`))
    (if (not (`self.EndlessCombustion`))
      (`self.BurningDuration`))
    (if (`self.Pressurized`)
      (`self.Explosion`))))

(fn `IgnitionLifetime`
  (bind _ignitiontimeline (`self.IgnitionTimeline`))
  (`TimelineComponent.SetPlayRate` _ignitiontimeline (/ (`TimelineComponent.GetTimelineLength` _ignitiontimeline) (`self.IgnitionTimeRequitement`))))

(fn `IgnitionMultiplier`
  (bind _ignitiontimeline (`self.IgnitionTimeline`))
  (bind _debugshowignitionmodifier (`self.DebugShowIgnitionModifier`))
  (bind _returnvalue (`KismetArrayLibrary.Array_Length` (`self.CombustibleVolumes`)))
  (bind _returnvalue_2 (`TimelineComponent.GetTimelineLength` _ignitiontimeline))
  (bind _returnvalue_3 (/ _returnvalue_2 (`self.IgnitionTimeRequitement`)))
  (bind _returnvalue_4 (select `bool` (>= _returnvalue 2) :`false` _returnvalue_3 :`true` (* _returnvalue_3 (* (`self.IgnitionSpeedMultiplier`) _returnvalue)) :!type "Float (single-precision)"))
  (`TimelineComponent.SetPlayRate` _ignitiontimeline _returnvalue_4)
  (`KismetSystemLibrary.PrintString` (`KismetStringLibrary.Concat_StrStr` (`KismetStringLibrary.Conv_IntToString` _returnvalue) "  OVERLAP ACTOR  ---  " (`KismetStringLibrary.Conv_DoubleToString` (* _returnvalue_2 _returnvalue_4)) " Seconds") _debugshowignitionmodifier true (struct :`R` 0.98018 :`B` 1.0 :`A` 1.0) 8.0)
  (for (_array_element _array_index) (`self.CombustibleVolumes`)
    (`KismetSystemLibrary.PrintString` (`KismetStringLibrary.Concat_StrStr` "INDEX " (`KismetStringLibrary.Conv_IntToString` _array_index) "   ---   " (`KismetSystemLibrary.GetDisplayName` _array_element)) _debugshowignitionmodifier true (struct :`G` 1.0 :`B` 0.207824 :`A` 1.0) 8.0)))

(fn `IgnitionReverted`
  (set `self.Burning` false)
  (`self.Disable Propagation`)
  (`ActorComponent.Deactivate` (`self.NS_IgniteSmoke`))
  (`ActorComponent.Deactivate` (`self.NS_BurningSmoke`))
  (`ActorComponent.Deactivate` (`self.NS_Fire`))
  (`self.CancelTextAnim`))

(fn `SetPropagationSize`
  (params (DoNotScale :type Boolean))
  (`SceneComponent.SetRelativeScale3D` (`self.Root_Propagation`) (* (select `bool` DoNotScale :`false` (select `/Game/Blueprint/CombustibleObject/E_FirePropagationSize` (`self.PropagationSize`) :`NewEnumerator0` (1.125 1.125 1.25) :`NewEnumerator1` (1.25 1.25 1.5) :`NewEnumerator2` (1.5 1.5 1.75) :`NewEnumerator3` (1.75 1.75 2.0) :`NewEnumerator4` (2.0 2.0 2.25) :`NewEnumerator5` (2.25 2.25 2.5) :`NewEnumerator6` (2.5 2.5 2.75) :`NewEnumerator7` (`self.CustomPropagationSize`)) :`true` (1.0 1.0 1.0)) (1.0 1.0 1.0))))

(fn `Stop Text Animation`
  (params (`Ignition Text Anim` :type Boolean :default true) (`Extinction Text Anim` :type Boolean :default true) (` Burning Text Anim` :type Boolean :default true))
  (if `Ignition Text Anim`
    (`self.Stop Ignite Text Animation`))
  (if `Extinction Text Anim`
    (`self.Stop Extinction Text Animation`))
  (if ` Burning Text Anim`
    (`self.Stop Burning Text Animation`)))

(fn `UserConstructionScript`
  (bind _burninglifetimeline (`self.BurningLifeTimeline`))
  (bind _sm_combustibleobject (`self.SM_CombustibleObject`))
  (`self.IgnitionLifetime`)
  (`TimelineComponent.SetPlayRate` _burninglifetimeline (/ (`TimelineComponent.GetTimelineLength` _burninglifetimeline) (`self.BurningTimeDuration`)))
  (bind _returnvalue (`PrimitiveComponent.CreateDynamicMaterialInstance` _sm_combustibleobject 0 (`PrimitiveComponent.GetMaterial` _sm_combustibleobject 0) "None"))
  (set `self.BurningShader` _returnvalue)
  (`MaterialInstanceDynamic.SetScalarParameterValue` (`self.BurningShader`) "Range" 0.0)
  (`NiagaraComponent.SetAsset` (`self.NS_IgniteSmoke`) (`self.PS_SmokeIgnite`) true)
  (`ParticleSystemComponent.SetTemplate` (`self.CPS_Explosion`) (`self.PS Explosion`))
  (`NiagaraComponent.SetAsset` (`self.NS_Fire`) (`self.PS Fire`) true)
  (`NiagaraComponent.SetAsset` (`self.NS_BurningSmoke`) (`self.PS_BurningSmoke`) true)
  (`NiagaraComponent.SetAsset` (`self.NS_BurntOutSmoke`) (`self.PS_SmokeBurntOut`) true)
  (`SceneComponent.SetHiddenInGame` (`self.Progation Collision Box`) (not (`self.DebugCollisionVisibility`)) false)
  (`self.SetPropagationSize` (`self.Debug Propagation Scale`)))