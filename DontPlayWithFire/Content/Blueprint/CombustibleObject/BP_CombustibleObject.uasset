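; Combustible actor that ignites, burns, spreads fire to other combustibles, and burns out unless set to endless.
; Timelines drive dynamic fire materials, radial progress, status text and a propagation box that ignites overlapping combustibles.
; Overlapping dowsing volumes reverse the ignition timeline to extinguish it and block propagation.
; Pressurized objects explode on ignition, swapping mesh, launching characters and pushing nearby combustibles while raising their ignition value.
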(event `Initiate DowsingProtocol`
  ;[1 0 0.06535 0.5] Dowsing Logic
  (`self.DowsingProtocol`))

(event `self.Extinction Collision.OnComponentBeginOverlap`
  (params (OverlappedComponent :type "PrimitiveComponent Object Reference") (OtherActor :type "Actor Object Reference") (OtherComp :type "PrimitiveComponent Object Reference") (OtherBodyIndex :type Integer) (bFromSweep :type Boolean) (SweepResult :type "HitResult Structure (by ref)"))
  ;[1 0 0.06535 0.5] Dowsing Logic
  (bind _asbp_master_dowsing_volume (cast `/Game/Blueprint/DowsingVolumes/BP_Master_DowsingVolume` OtherActor))
  (`KismetArrayLibrary.Array_Add` (`self.DowsingVolumes`) _asbp_master_dowsing_volume)
  (`self.Initiate DowsingProtocol`))

(event `Stop Dowsing Protocol`
  ;[1 0 0.06535 0.5] Dowsing Logic
  (`/Engine/EditorBlueprintResources/StandardMacros.IsValid` (`|GetArrayItem` (`self.DowsingVolumes`))
    (:`Is Not Valid`
      (set `self.Dowsed` false)
      (`self.Cancelled Ignition`))))

(event `self.Extinction Collision.OnComponentEndOverlap`
  (params (OverlappedComponent :type "PrimitiveComponent Object Reference") (OtherActor :type "Actor Object Reference") (OtherComp :type "PrimitiveComponent Object Reference") (OtherBodyIndex :type Integer))
  ;[1 0 0.06535 0.5] Dowsing Logic
  (bind _asbp_master_dowsing_volume (cast `/Game/Blueprint/DowsingVolumes/BP_Master_DowsingVolume` OtherActor))
  (`KismetArrayLibrary.Array_RemoveItem` (`self.DowsingVolumes`) _asbp_master_dowsing_volume)
  (`self.Stop Dowsing Protocol`))

(event `self.ReceiveBeginPlay`
  ;[0 0.4851 1 0.5] Begin Play
  (`PrimitiveComponent.SetCollisionEnabled` (`self.Progation Collision Box`) "NoCollision")
  (`BoxComponent.SetBoxExtent` (`self.Progation Collision Box`) (`self.ZeroPropagationSize`) false)
  (if (`self.IgnitionAtStart`)
    (`self.Ignite`)))

(event `Enable Propagation`
  ;[1 0 0.06535 0.5] Propagation Logic
  (`PrimitiveComponent.SetCollisionEnabled` (`self.Progation Collision Box`) "QueryOnly"))

(event `self.Progation Collision Box.OnComponentBeginOverlap`
  (params (OverlappedComponent :type "PrimitiveComponent Object Reference") (OtherActor :type "Actor Object Reference") (OtherComp :type "PrimitiveComponent Object Reference") (OtherBodyIndex :type Integer) (bFromSweep :type Boolean) (SweepResult :type "HitResult Structure (by ref)"))
  ;[1 0 0.06535 0.5] Propagation Logic
  (if (not (`self.Dowsed`))
    (bind _asbp_combustible_object (cast `/Game/Blueprint/CombustibleObject/BP_CombustibleObject` OtherActor))
    (`self.Ignite` _asbp_combustible_object)))

(event `Disable Propagation`
  ;[1 0 0.06535 0.5] Propagation Logic
  (`PrimitiveComponent.SetCollisionEnabled` (`self.Progation Collision Box`) "NoCollision"))

(event `ExtinctionTextAnim`
  ;[1.5 1.093 0 0.5] Text Update Anim
  (`|ExecutionSequence`
    (:`then_0`
      (`Timeline|IgniteTextAnimation` :!via `Stop` :!label _label
        (:`NewTrack_0`
          (set `self.TextStatus` "Igniting"))
        (:`NewTrack_1`
          (set `self.TextStatus` "Igniting."))
        (:`NewTrack_2`
          (set `self.TextStatus` "Igniting.."))
        (:`NewTrack_3`
          (set `self.TextStatus` "Igniting...")))
      (`TextRenderComponent.K2_SetText` (`self.Txt_ObjectStatus`) (`self.TextStatus`)))
    (:`then_1`
      (`Timeline|BurningTextAnimation` :!via `Stop` :!label _label_2
        (:`NewTrack_0`
          _)
        (:`NewTrack_1`
          _)
        (:`NewTrack_2`
          _)
        (:`NewTrack_3`
          _))
      (bind _isa (`/Engine/EditorBlueprintResources/StandardMacros.FlipFlop`)
        (:`A`
          _)
        (:`B`
          _))
      (`SceneComponent.SetVisibility` (`self.Txt_ObjectStatus`) _isa false))
    (:`then_2`
      (`SceneComponent.SetVisibility` (`self.Txt_ObjectStatus`) true false)
      (`Timeline|Timeline` :!label _label_3
        (:`NewTrack_0`
          (set `self.TextStatus` "Extiguishing"))
        (:`NewTrack_1`
          (set `self.TextStatus` "Extiguishing."))
        (:`NewTrack_2`
          (set `self.TextStatus` "Extiguishing.."))
        (:`NewTrack_3`
          (set `self.TextStatus` "Extiguishing...")))
      (`TextRenderComponent.K2_SetText` (`self.Txt_ObjectStatus`) (`self.TextStatus`)))))

(event `Ignite`
  ;[1 0 0.06535 0.5] Ignition
  (if (not (`self.Burning`))
    (`self.IgniteAnimation`)))

(event `self.Progation Collision Box.OnComponentEndOverlap`
  (params (OverlappedComponent :type "PrimitiveComponent Object Reference") (OtherActor :type "Actor Object Reference") (OtherComp :type "PrimitiveComponent Object Reference") (OtherBodyIndex :type Integer))
  ;[1 0 0.06535 0.5] Propagation Logic
  (if (not (`self.Dowsed`))
    (bind _asbp_combustible_object (cast `/Game/Blueprint/CombustibleObject/BP_CombustibleObject` OtherActor))
    (`self.Cancelled Ignition` _asbp_combustible_object)))

(event `Cancelled Ignition`
  ;[1 0 0.06535 0.5] Ignition
  (if (not (`self.Burning`))
    (`self.CancelledIgniteAnimation`)))

(event `Reverse Ignition`
  ;[1 0 0.06535 0.5] Ignition
  (if (`self.Burning`)
    (set `self.Burning` false))
  (`self.ReverseIgniteAnimation`))

(event `IgniteTextAnim`
  ;[1.5 1.093 0 0.5] Text Update Anim
  (`|ExecutionSequence`
    (:`then_0`
      (goto _label_2 :!via `Stop`))
    (:`then_1`
      (goto _label_3 :!via `Stop`))
    (:`then_2`
      (`SceneComponent.SetVisibility` (`self.Txt_ObjectStatus`) true false)
      (goto _label))))

(event `IgniteAnimation`
  ;[1.5 1.093 0 0.5] Ignition Animation
  (`self.IgniteTextAnim`)
  (bind (_direction _ignitionalpha) (`Timeline|IgnitionTimeline` :`NewTime` (`self.IgnitionValue`) :!label _label_4)
    (:`Update`
      (set `self.IgnitionValue` _ignitionalpha)
      (`MaterialInstanceDynamic.SetScalarParameterValue` (`self.BurningShader`) "FireVisibility" (`KismetMathLibrary.Lerp` 0.0 1.0 _ignitionalpha))
      (`MaterialInstanceDynamic.SetScalarParameterValue` (`self.Radial Progressbar`) "Percent" (`KismetMathLibrary.Lerp` 0.0 1.0 _ignitionalpha))
      (`BoxComponent.SetBoxExtent` (`self.Progation Collision Box`) (`KismetMathLibrary.VLerp` (`self.ZeroPropagationSize`) (`self.MinimalPropagationationSize`) _ignitionalpha) true))
    (:`Finished`
      (switch `ETimelineDirection` _direction
        (:`Forward`
          (`self.IgnitionComplete`)
          (`KismetSystemLibrary.Delay` 0.25)
          (`SceneComponent.SetVisibility` (`self.MaterialBillboard`) false false))
        (:`Backward`
          (`self.IgnitionReverted`)
          (`KismetSystemLibrary.Delay` 0.25)
          (`SceneComponent.SetVisibility` (`self.MaterialBillboard`) false false))))))

(event `CancelledIgniteAnimation`
  ;[1.5 1.093 0 0.5] Ignition Animation
  (`self.CancelTextAnim`)
  (goto _label_4 :!via `Stop`))

(event `CancelTextAnim`
  ;[1.5 1.093 0 0.5] Text Update Anim
  (`|ExecutionSequence`
    (:`then_0`
      (goto _label :!via `Stop`))
    (:`then_1`
      (goto _label_2 :!via `Stop`))
    (:`then_2`
      (goto _label_3 :!via `Stop`))))

(event `ReverseIgniteAnimation`
  ;[1.5 1.093 0 0.5] Ignition Animation
  (`self.ExtinctionTextAnim`)
  (`SceneComponent.SetVisibility` (`self.MaterialBillboard`) true false)
  (goto _label_4 :!via `Reverse`))

(event `BurningTextAnim`
  ;[1.5 1.093 0 0.5] Text Update Anim
  (`|ExecutionSequence`
    (:`then_0`
      (goto _label :!via `Stop`))
    (:`then_1`
      (goto _label_3 :!via `Stop`))
    (:`then_2`
      (set `self.TextStatus` "Burning!")
      (`TextRenderComponent.K2_SetText` (`self.Txt_ObjectStatus`) (`self.TextStatus`))
      (goto _label_2))))

(event `Burn Out`
  ;[1.5 1.093 0 0.5] Burnout Animation
  (`self.BurntOutVFX`)
  (`self.CancelTextAnim`)
  (set `self.CurrentPropagationationSize` (`BoxComponent.GetScaledBoxExtent` (`self.Progation Collision Box`)))
  (bind (_direction _burnoutlerp) (`Timeline|BurnoutTimeline`)
    (:`Update`
      (`MaterialInstanceDynamic.SetVectorParameterValue` (`self.BurningShader`) "FireColor" (`KismetMathLibrary.LinearColorLerp` (`self.CurrentBurningColor`) (struct :`A` 2.0) _burnoutlerp))
      (`BoxComponent.SetBoxExtent` (`self.Progation Collision Box`) (`KismetMathLibrary.VLerp` (`self.CurrentPropagationationSize`) (`self.ZeroPropagationSize`) _burnoutlerp) true))
    (:`Finished`
      (`self.Disable Propagation`))))

(event `BurningAnimation`
  ;[1.5 1.093 0 0.5] Burning Animation Loop
  (`self.BurningTextAnim`)
  (bind (_direction _burningshaderlerp) (`Timeline|BurningTimeline` :!via `PlayFromStart` :!label _label_5)
    (:`Update`
      (bind _returnvalue (`KismetMathLibrary.LinearColorLerp` (struct :`R` 1.0 :`G` 0.564712 :`A` 1.0) (struct :`R` 0.375 :`G` 0.211767 :`A` 2.0) _burningshaderlerp))
      (set `self.CurrentBurningColor` _returnvalue)
      (`MaterialInstanceDynamic.SetVectorParameterValue` (`self.BurningShader`) "FireColor" _returnvalue)
      (`BoxComponent.SetBoxExtent` (`self.Progation Collision Box`) (`KismetMathLibrary.VLerp` (`self.MinimalPropagationationSize`) (`self.MaximalPropagationationSize`) _burningshaderlerp) true))))

(event `Extinguish Succeed`
  ;[1.5 1.093 0 0.5] Burning Animation Loop
  (goto _label_5 :!via `Stop`))

(event `BurningDuration`
  ;[1.5 1.093 0 0.5] Burning Animation Loop
  (`KismetSystemLibrary.Delay` (`self.BurningDurationDelay`))
  (`|ExecutionSequence`
    (:`then_0`
      (goto _label_5 :!via `Stop`))
    (:`then_1`
      (`self.Burn Out`))))

(fn `BlastCharacter`
  (params (Character :type "Character Object Reference") (ExplosionLocation :type "Vector Structure") (BlastRadius :type "Float (single-precision)"))
  (bind _returnvalue (`self.K2_GetActorLocation` Character))
  (bind _returnvalue_2 (`KismetMathLibrary.Vector_Distance` _returnvalue ExplosionLocation))
  (if (<= _returnvalue_2 BlastRadius)
    (`Character.LaunchCharacter` Character (+ (* (`KismetMathLibrary.GetDirectionUnitVector` ExplosionLocation _returnvalue) (* (/ BlastRadius _returnvalue_2) (* (`self.ExplosionStrength`) 0.1))) (0.0 0.0 250.0)) false false)))

(fn `BlastObject`
  (params (CombustibleObject :type "/Game/Blueprint/CombustibleObject/BP_CombustibleObject Object Reference") (ExplosionLocation :type "Vector Structure") (BlastRadius :type "Float (single-precision)"))
  (bind _explosiondamage (`self.ExplosionDamage`))
  (if (not (== CombustibleObject self))
    (`PhysicsObjectBlueprintLibrary.ApplyRadialImpulse` (`/Game/Blueprint/CombustibleObject/BP_CombustibleObject.SM_CombustibleObject` CombustibleObject) ExplosionLocation BlastRadius (`self.ExplosionStrength`) "RIF_Linear" false 0.0 true)
    (bind _output_get (set `/Game/Blueprint/CombustibleObject/BP_CombustibleObject.IgnitionValue` (`KismetMathLibrary.FClamp` (+ (`/Game/Blueprint/CombustibleObject/BP_CombustibleObject.IgnitionValue` CombustibleObject) _explosiondamage (* _explosiondamage (/ BlastRadius (`KismetMathLibrary.Vector_Distance` ExplosionLocation (`self.K2_GetActorLocation` CombustibleObject)))))) CombustibleObject))
    (if (>= _output_get 1.0)
      (`self.IgnitionComplete` CombustibleObject))))

(fn `BurntOutVFX`
  (`ActorComponent.Deactivate` (`self.CPS_Smoke`))
  (`ActorComponent.Deactivate` (`self.CPS_Fire`))
  (`ActorComponent.Activate` (`self.CPS_SmokeBurntOut`) false))

(fn `DowsingProtocol`
  (set `self.Dowsed` true)
  (`self.Reverse Ignition`))

(fn `Explosion`
  (bind _exploded_mesh (`self.Exploded Mesh`))
  (bind _blastradiuscapsule (`self.BlastRadiusCapsule`))
  (bind _returnvalue (`SceneComponent.K2_GetComponentLocation` (`self.Progation Collision Box`)))
  (set `self.HasExploded` true)
  (`ActorComponent.Activate` (`self.CPS_Explosion`) false)
  (`/Engine/EditorBlueprintResources/StandardMacros.IsValid` _exploded_mesh
    (:`Is Valid`
      (`StaticMeshComponent.SetStaticMesh` (`self.SM_CombustibleObject`) _exploded_mesh))
    (:`Is Not Valid`
      _))
  (bind _outactors (`KismetSystemLibrary.SphereOverlapActors` _returnvalue _blastradiuscapsule (`self.Object Types`) null (`|MakeArray` self :!type "Actor Object Reference")))
  (for _array_element _outactors
    (bind _asbp_combustible_object (cast `/Game/Blueprint/CombustibleObject/BP_CombustibleObject` _array_element)
      (:`then`
        (`self.BlastObject` _asbp_combustible_object _returnvalue _blastradiuscapsule))
      (:`CastFailed`
        (bind _ascharacter (cast `Character` _array_element))
        (`self.BlastCharacter` _ascharacter _returnvalue _blastradiuscapsule)))))

(fn `IgnitionComplete`
  (if (not (`self.HasExploded`))
    (set `self.Burning` true)
    (`self.Enable Propagation`)
    (`self.BurningAnimation`)
    (`ActorComponent.Activate` (`self.CPS_Smoke`) false)
    (`ActorComponent.Activate` (`self.CPS_Fire`) false)
    (if (not (`self.EndlessCombustion`))
      (`self.BurningDuration`))
    (if (`self.Pressurized`)
      (`self.Explosion`))))

(fn `IgnitionReverted`
  (set `self.Burning` false)
  (`self.Disable Propagation`)
  (`ActorComponent.Deactivate` (`self.CPS_Fire`))
  (`ActorComponent.Deactivate` (`self.CPS_Smoke`))
  (`self.CancelTextAnim`))

(fn `UserConstructionScript`
  (bind _sm_combustibleobject (`self.SM_CombustibleObject`))
  (`TimelineComponent.SetPlayRate` (`self.IgnitionTimeline`) (`self.IgnitionPlayRate`))
  (bind _returnvalue (`PrimitiveComponent.CreateDynamicMaterialInstance` _sm_combustibleobject 0 (`PrimitiveComponent.GetMaterial` _sm_combustibleobject 0) "None"))
  (set `self.BurningShader` _returnvalue)
  (bind _returnvalue_2 (`PrimitiveComponent.CreateDynamicMaterialInstance` (`self.MaterialBillboard`) 0 "/Game/LevelPrototyping/Materials/Instance/MI_RadialProgressBar.MI_RadialProgressBar" "None"))
  (set `self.Radial Progressbar` _returnvalue_2)
  (`ParticleSystemComponent.SetTemplate` (`self.CPS_Explosion`) (`self.PS Explosion`))
  (`ParticleSystemComponent.SetTemplate` (`self.CPS_Fire`) (`self.PS Fire`))
  (`ParticleSystemComponent.SetTemplate` (`self.CPS_Smoke`) (`self.PS Smoke`))
  (`ParticleSystemComponent.SetTemplate` (`self.CPS_SmokeBurntOut`) (`self.PS Smoke Burnt Out`))
  (`SceneComponent.SetHiddenInGame` (`self.Progation Collision Box`) (not (`self.DebugCollisionVisibility`)) false))