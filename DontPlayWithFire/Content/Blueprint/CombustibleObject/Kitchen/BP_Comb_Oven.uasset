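; BP_Comb_Oven is a kitchen oven prop assembled from two combustible-object child actors, the oven body and its door.
; On BeginPlay it casts both child actors to BP_Master_CombustibleObject and stores them as oven and door references.
; It then binds their static meshes to a PhysicsConstraint at runtime, physically linking the door to the body.
; If either cast fails, the constraint is never bound.
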(event `self.ReceiveBeginPlay`
  (bind _asbp_master_combustible_object (cast `/Game/Blueprint/CombustibleObject/BP_Master_CombustibleObject` (`ChildActorComponent.ChildActor` (`self.BP_Comb_OverPart_01`))))
  (set `self.As BP Oven` _asbp_master_combustible_object)
  (bind _asbp_master_combustible_object_2 (cast `/Game/Blueprint/CombustibleObject/BP_Master_CombustibleObject` (`ChildActorComponent.ChildActor` (`self.BP_Comb_OverPart_02`))))
  (set `self.As BP Oven Door` _asbp_master_combustible_object_2)
  (`PhysicsConstraintComponent.SetConstrainedComponents` (`self.PhysicsConstraint`) (`/Game/Blueprint/CombustibleObject/BP_Master_CombustibleObject.SM_CombustibleObject` (`self.As BP Oven`)) "None" (`/Game/Blueprint/CombustibleObject/BP_Master_CombustibleObject.SM_CombustibleObject` (`self.As BP Oven Door`)) "None"))

(fn `UserConstructionScript`)