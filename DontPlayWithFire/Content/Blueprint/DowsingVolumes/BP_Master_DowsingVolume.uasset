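; Master Blueprint for a foam blob projectile that wobbles in flight and self-destructs after three seconds without landing.
; On overlap, a sphere trace along its velocity stops it, snaps it to the surface normal and disables collision.
; It then immediately shrinks, sinks and is destroyed via a timeline.
; Flattening, wall-drip, ceiling-drop and the surface-angle macro exist but are not wired in.
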(event `self.ReceiveBeginPlay`
  (bind _returnvalue (`KismetMathLibrary.RandomFloatInRange` 0.25 0.6))
  (bind _projectilemovement (`self.ProjectileMovement`))
  ;[0 0.1529 1 0.5] Begin Play
  (set `ProjectileMovementComponent.InitialSpeed` (* (`ProjectileMovementComponent.InitialSpeed` _projectilemovement) (`KismetMathLibrary.RandomFloatInRange` 1.0 1.25)) _projectilemovement)
  (bind _output_get (set `self.InitialScale` (`KismetMathLibrary.MakeVector` _returnvalue _returnvalue _returnvalue)))
  (`SceneComponent.SetRelativeScale3D` (`self.SM_Foam`) _output_get)
  (`self.AnimAirBlob`)
  (`KismetSystemLibrary.Delay` 3.0)
  (if (`self.IsStillInAir`)
    (`self.K2_DestroyActor`)))

(event `AnimAirBlob`
  (bind (_initialscale_x _initialscale_y _initialscale_z) (`KismetMathLibrary.BreakVector` (`self.InitialScale`)))
  (bind _returnvalue (`KismetMathLibrary.RandomFloatInRange` (`self.MinMultiplier`) (`self.MaxMultiplier`)))
  ;[2 1.759 0.1667 0.5] In Air Animation
  (bind (_direction _blobbyinairanimation) (`Timeline|In Air Blob` :!label _label)
    (:`Update`
      (set `self.Blobby in Air Animation` _blobbyinairanimation)
      (bind _output_get (set `self.CurrentScale` (`KismetMathLibrary.VLerp` (`self.InitialScale`) (`self.BlobRandomScale`) _blobbyinairanimation)))
      (`SceneComponent.SetRelativeScale3D` (`self.SM_Foam`) _output_get))
    (:`BeginingLoop`
      (set `self.BlobRandomScale` (`KismetMathLibrary.MakeVector` (* _initialscale_x _returnvalue) (* _initialscale_y _returnvalue) (* _initialscale_z _returnvalue))))))

(event `StopAnimAirBlob`
  ;[2 1.759 0.1667 0.5] In Air Animation
  (set `self.CurrentScale` (`KismetMathLibrary.VLerp` (`self.InitialScale`) (`self.BlobRandomScale`) (`self.Blobby in Air Animation`)))
  (goto _label :!via `Stop`))

(event `AnimFlatBlob`
  ;[2 1.759 0.1667 0.5] Landing Flat Animation
  (`PrimitiveComponent.SetCollisionEnabled` (`self.SphereCollision`) "NoCollision")
  (`/Engine/EditorBlueprintResources/StandardMacros.DoOnce` false
    (:`Completed`
      (`self.Anim Death`))))

(event `Anim Death`
  (bind _flatmodifierxy (`self.FlatModifierXY`))
  (bind (_currentscale_x _currentscale_y _currentscale_z) (`KismetMathLibrary.BreakVector` (`self.CurrentScale`)))
  ;[2 1.759 0.1667 0.5] Drying Out Animation
  (`TimelineComponent.SetPlayRate` (`self.DeathAnimTimeline`) (`KismetMathLibrary.RandomFloatInRange` 0.9 1.2))
  (bind (_direction _newtrack_0) (`Timeline|DeathAnimTimeline`)
    (:`Update`
      (`SceneComponent.SetRelativeScale3D` (`self.SM_Foam`) (`KismetMathLibrary.VLerp` (`KismetMathLibrary.MakeVector` (* _currentscale_x _flatmodifierxy) (* _currentscale_y _flatmodifierxy) (* _currentscale_z _flatmodifierxy)) (0.01 0.01 0.01) _newtrack_0))
      (`self.K2_SetActorLocation` (- (`self.K2_GetActorLocation`) (0.0 0.0 0.35))))
    (:`Finished`
      (`self.K2_DestroyActor`))))

(event `AnimFalling`
  (bind (_initialscale_x _initialscale_y _initialscale_z) (`KismetMathLibrary.BreakVector` (`self.InitialScale`)))
  (bind _fallingmodifierxy (`self.FallingModifierXY`))
  (bind (_direction _newtrack_0) (`Timeline|Timeline_0` :!via `PlayFromStart` :!label _label_2)
    (:`Update`
      (bind _returnvalue (`KismetMathLibrary.VLerp` (`self.CurrentScale`) (`KismetMathLibrary.MakeVector` (* _initialscale_x _fallingmodifierxy) (* _initialscale_y _fallingmodifierxy) (* _initialscale_z (`self.FallingModifierZ`))) _newtrack_0))
      (set `self.CurrentScale` _returnvalue)
      (`SceneComponent.SetRelativeScale3D` (`self.SM_Foam`) _returnvalue))))

(event `StopAnimFalling`
  (goto _label_2 :!via `Stop`))

(event `Trigger Projectile Tick`
  (bind _returnvalue (`KismetSystemLibrary.K2_SetTimerDelegate` (delegate `ProjectileUpdate`) 0.0001 true true))
  (set `self.ProjectileTick` _returnvalue))

(event `ProjectileUpdate`)

(event `self.SphereCollision.OnComponentBeginOverlap`
  (params (OverlappedComponent :type "PrimitiveComponent Object Reference") (OtherActor :type "Actor Object Reference") (OtherComp :type "PrimitiveComponent Object Reference") (OtherBodyIndex :type Integer) (bFromSweep :type Boolean) (SweepResult :type "HitResult Structure (by ref)"))
  (bind _returnvalue (`self.K2_GetActorLocation`))
  (bind (_bblockinghit _binitialoverlap _time _distance _location _impactpoint _normal) (`GameplayStatics.BreakHitResult` (`self.Out Hit`)))
  (bind _output_get (set `self.Hit Actor` OtherActor))
  (bind (_outhits _returnvalue_2) (`KismetSystemLibrary.SphereTraceMulti` _returnvalue (+ _returnvalue (* (`KismetMathLibrary.GetDirectionUnitVector` _returnvalue (`self.GetVelocity`)) 15.0)) (* (`SphereComponent.SphereRadius` (`self.SphereCollision`)) 2.0) "TraceTypeQuery1" true (`|MakeArray` (`self.GetOwner`) (cast `/Game/Blueprint/DowsingVolumes/BP_Master_DowsingVolume` _output_get :!pure true) (`GameplayStatics.GetPlayerCharacter` 0) :!type "Actor Object Reference")))
  (for _array_element _outhits :!label _label_3
    (set `self.Out Hit` _array_element)
    (if _returnvalue_2
      (if (and (or (not (== (`self.GetOwner`) _output_get)) (not (== _output_get (cast `/Game/Blueprint/DowsingVolumes/BP_Master_DowsingVolume` _output_get :!pure true)))) _bblockinghit)
        (set `self.IsStillInAir` false)
        (`ProjectileMovementComponent.StopSimulating` (`self.ProjectileMovement`) (`self.Out Hit`))
        (`self.StopAnimAirBlob`)
        (`self.AnimFlatBlob`)
        (if (not (`self.HasImpacted`))
          (bind _output_get_2 (set `self.ImpactAngle` (`KismetMathLibrary.MakeRotFromZ` _normal)))
          (`self.K2_SetActorLocationAndRotation` _impactpoint _output_get_2)
          (set `self.HasImpacted` true)
          (`self.stop loop`))))))

(event `stop loop`
  (goto _label_3 :!via `Break`))

(event `DripWallUpdate`
  (bind _returnvalue (`self.K2_GetActorLocation`))
  (`self.K2_SetActorLocationAndRotation` (- (`self.K2_GetActorLocation`) (* (`KismetMathLibrary.GetRightVector` (`self.ImpactAngle`)) (`self.DrippingSpeed`))) (`self.K2_GetActorRotation`) true)
  (bind _outhit (`KismetSystemLibrary.LineTraceSingle` _returnvalue (- _returnvalue (* (`KismetMathLibrary.GetRightVector` (`self.ImpactAngle`)) 5.0)) "TraceTypeQuery1" false (`|MakeArray` self (cast `/Game/Blueprint/DowsingVolumes/BP_Master_DowsingVolume` (`self.Hit Actor`) :!pure true) :!type "Actor Object Reference") "ForDuration" true (struct :`R` 1.0 :`B` 0.836866 :`A` 1.0) (struct :`G` 1.0 :`A` 1.0) 0.1))
  (bind (_bblockinghit _binitialoverlap _time _distance _location _impactpoint _normal _impactnormal _physmat _hitactor) (`GameplayStatics.BreakHitResult` _outhit))
  (if (and _bblockinghit (not (`.bSuccess` (cast `/Game/Blueprint/DowsingVolumes/BP_Master_DowsingVolume` _hitactor :!pure true))))
    (bind _returnvalue_2 (`KismetMathLibrary.MakeRotFromZ` _normal))
    (if (not (== (`self.ImpactAngle`) _returnvalue_2 :`ErrorTolerance` 0.5))
      (set `self.ImpactAngle` _returnvalue_2))))

(event `DropCeilingUpdate`
  (bind (_returnvalue_x _returnvalue_y _returnvalue_z) (`KismetMathLibrary.BreakVector` (`self.K2_GetActorLocation`)))
  (bind _returnvalue (`self.K2_GetActorLocation`))
  (bind _output_get (set `self.Falling Speed` (`KismetMathLibrary.FClamp` (* (`self.Falling Speed`) (`self.Falling Speed Multiplier`)) 2.0 15.0)))
  (bind _outhit (`KismetSystemLibrary.LineTraceSingle` (- _returnvalue (0.0 0.0 1.0)) (- _returnvalue (`KismetMathLibrary.MakeVector` 0.0 0.0 _output_get)) "TraceTypeQuery1" false (`|MakeArray` self (cast `/Game/Blueprint/DowsingVolumes/BP_Master_DowsingVolume` (`self.Hit Actor`) :!pure true) :!type "Actor Object Reference") "ForDuration" true (struct :`R` 1.0 :`B` 0.836866 :`A` 1.0) (struct :`G` 1.0 :`A` 1.0) 0.1))
  (bind (_bblockinghit _binitialoverlap _time _distance _location _impactpoint _normal _impactnormal _physmat _hitactor) (`GameplayStatics.BreakHitResult` _outhit))
  (if (and _bblockinghit (not (`.bSuccess` (cast `/Game/Blueprint/DowsingVolumes/BP_Master_DowsingVolume` _hitactor :!pure true))))
    (`self.K2_SetActorLocationAndRotation` _impactpoint (struct) true)
    (else
      (`self.K2_SetActorLocationAndRotation` (`KismetMathLibrary.MakeVector` _returnvalue_x _returnvalue_y (- _returnvalue_z (`self.Falling Speed`))) (struct) true))))

(fn `Pause Timer Drip Wall Update`
  (bind _timerdripwallupdate (`self.TimerDripWallUpdate`))
  (if (`KismetSystemLibrary.K2_IsValidTimerHandle` _timerdripwallupdate)
    (`KismetSystemLibrary.K2_PauseTimerHandle` _timerdripwallupdate)))

(fn `Pause Timer Drop Ceiling Update`
  (bind _timerdropceilingupdate (`self.TimerDropCeilingUpdate`))
  (if (`KismetSystemLibrary.K2_IsValidTimerHandle` _timerdropceilingupdate)
    (`KismetSystemLibrary.K2_PauseTimerHandle` _timerdropceilingupdate)
    (`self.StopAnimFalling`)))

(fn `UserConstructionScript`)