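; BP_PickUp_Axe is the world pickup for the axe, which a fireman player swaps for an equipment actor.
; PickupBehavior spawns SpawnActorClass at the player's location, with the player as owner and instigator.
; If the spawn casts to BP_Master_Equipement, it stores this pickup's class as DropActorClass for dropping, clears the player's PickupObject and destroys itself.
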(event `self.PickupBehavior`
  (params (PlayerFireman :type "/Game/Blueprint/Character/Master/BP_GenericCharacter Object Reference"))
  (bind _returnvalue (`|SpawnActorFromClass` (`self.SpawnActorClass`) (`KismetMathLibrary.MakeTransform` (`self.K2_GetActorLocation` PlayerFireman)) "Undefined" "MultiplyWithRoot" PlayerFireman PlayerFireman))
  (bind _asbp_master_equipement (cast `/Game/Blueprint/Equipement/Master/BP_Master_Equipement` _returnvalue))
  (set `/Game/Blueprint/Equipement/Master/BP_Master_Equipement.DropActorClass` (`GameplayStatics.GetObjectClass` self) _asbp_master_equipement)
  (set `/Game/Blueprint/Character/Master/BP_GenericCharacter.PickupObject` null PlayerFireman)
  (`self.K2_DestroyActor`))

(fn `UserConstructionScript`
  (`parent.UserConstructionScript`))