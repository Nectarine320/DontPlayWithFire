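; Ranged equipment master Blueprint that fires dowsing volumes toward the point under the screen center.
; ShootingRaytrace traces from screen center, falling back to a distant point on a miss, then retraces from the weapon's projectile bone.
; While the character is in shooting position, triggered input spawns a BP_Master_DowsingVolume at that bone, facing the aim point; the second trace's hit is unused.
; Shooting start and completion toggle the character's IsShooting flag.
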(event `self.ReceiveBeginPlay`
  (`parent.ReceiveBeginPlay`))

(event `Shooting Triggered`
  (bind _as_bp_generic_character (`self.As BP Generic Character`))
  ;[1 0 0.06535 0.5] Input Shooting
  (if (`/Game/Blueprint/Character/BP_GenericCharacter.InShootingPosition` (`self.As BP Generic Character`))
    (bind (_traceorigine _traceend) (`self.ShootingRaytrace`))
    (`|SpawnActorFromClass` "/Game/Blueprint/DowsingVolumes/BP_Master_DowsingVolume.BP_Master_DowsingVolume_C" (`KismetMathLibrary.MakeTransform` _traceorigine (`KismetMathLibrary.FindLookAtRotation` _traceorigine (+ _traceend (0.0 0.0 0.0)))) "Undefined" "MultiplyWithRoot" _as_bp_generic_character _as_bp_generic_character)))

(event `Shooting Started`
  ;[1 0 0.06535 0.5] Input Shooting
  (set `/Game/Blueprint/Character/BP_GenericCharacter.IsShooting` true (`self.As BP Generic Character`)))

(event `Shooting Completed`
  ;[1 0 0.06535 0.5] Input Shooting
  (set `/Game/Blueprint/Character/BP_GenericCharacter.IsShooting` false (`self.As BP Generic Character`)))

(fn `ShootingRaytrace`
  (returns (TraceOrigine :type "Vector Structure") (TraceEnd :type "Vector Structure") (OutHit :type "HitResult Structure") (`Return Value` :type Boolean))
  (bind _returnvalue (`GameplayStatics.GetPlayerController` 0))
  (bind (_sizex _sizey) (`PlayerController.GetViewportSize` _returnvalue))
  (bind _returnvalue_location (`KismetMathLibrary.BreakTransform` (`SkinnedMeshComponent.GetBoneTransform` (`self.SK_Equipment`) (`self.SourceOfBoneProjectile`) "RTS_World")))
  (bind (_worldposition _worlddirection) (`GameplayStatics.DeprojectScreenToWorld` _returnvalue (`KismetMathLibrary.MakeVector2D` (`KismetMathLibrary.Conv_IntToDouble` (/ _sizex 2)) (`KismetMathLibrary.Conv_IntToDouble` (/ _sizey 2)))))
  (bind _returnvalue_2 (+ _worldposition (* 5000.0 _worlddirection)))
  (bind (_outhit _returnvalue_3) (`KismetSystemLibrary.LineTraceSingle` _worldposition _returnvalue_2 "TraceTypeQuery1" false (`|MakeArray` (`GameplayStatics.GetPlayerPawn` 0) :!type "Actor Object Reference")))
  (bind _returnvalue_4 (select `bool` _returnvalue_3 :`false` _returnvalue_2 :`true` (`.ImpactPoint` (`GameplayStatics.BreakHitResult` _outhit))))
  (bind (_outhit_2 _returnvalue_5) (`KismetSystemLibrary.LineTraceSingle` _returnvalue_location _returnvalue_4 "TraceTypeQuery1" false (`|MakeArray` (`GameplayStatics.GetPlayerPawn` 0) :!type "Actor Object Reference") "None" true (struct :`R` 1.0 :`B` 0.836866 :`A` 1.0)))
  (return _returnvalue_location _returnvalue_4 _outhit_2 _returnvalue_5))

(fn `UserConstructionScript`
  (`parent.UserConstructionScript`))