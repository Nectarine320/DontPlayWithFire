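; Master melee equipment Blueprint that toggles the owning character's attacking state and damages destructible actors during a swing.
; A collision component attached to a mesh socket is enabled by PlayingChoppingAnim and disabled by EndingChoppingAnim, re-attaching each time.
; Component hits call HitRecieved on the other actor's BPC_Destructible.
; HitActorValidation uses AddUnique's returned index to allow one hit per actor, with the list cleared when each chop starts.
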(event `self.ReceiveBeginPlay`
  ;[0 0.1529 1 0.5] Begin Play / Initializer
  (`parent.ReceiveBeginPlay`)
  (`SceneComponent.K2_AttachToComponent` (`self.HitCollision`) (`self.SK_Equipment`) (`self.CollisionSocketName`) "SnapToTarget" "KeepWorld" "KeepWorld" true)
  (`PrimitiveComponent.SetCollisionEnabled` (`self.HitCollision`) "NoCollision"))

(event `HittingStart`
  (bind _as_bp_generic_character (`self.As BP Generic Character`))
  ;[1 0 0.06535 0.5] Input Shooting
  (if (not (`/Game/Blueprint/Character/Master/BP_GenericCharacter.IsAttacking` _as_bp_generic_character))
    (set `/Game/Blueprint/Character/Master/BP_GenericCharacter.IsAttacking` true _as_bp_generic_character)))

(event `HittingCancelled`
  ;[1 0 0.06535 0.5] Input Shooting
  (set `/Game/Blueprint/Character/Master/BP_GenericCharacter.IsAttacking` false (`self.As BP Generic Character`) :!label _label))

(event `HittingComplete`
  ;[1 0 0.06535 0.5] Input Shooting
  (goto _label))

(event `PlayingChoppingAnim`
  (`SceneComponent.K2_DetachFromComponent` (`self.HitCollision`) "KeepRelative" "KeepRelative" "KeepRelative" true)
  (`SceneComponent.K2_AttachToComponent` (`self.HitCollision`) (`self.SK_Equipment`) (`self.CollisionSocketName`) "SnapToTarget" "KeepWorld" "KeepWorld" true)
  (`PrimitiveComponent.SetCollisionEnabled` (`self.HitCollision`) "QueryAndPhysics")
  (`KismetArrayLibrary.Array_Clear` (`self.HittedActors`)))

(event `EndingChoppingAnim`
  (`PrimitiveComponent.SetCollisionEnabled` (`self.HitCollision`) "NoCollision")
  (`SceneComponent.K2_DetachFromComponent` (`self.HitCollision`) "KeepRelative" "KeepRelative" "KeepRelative" true)
  (`SceneComponent.K2_AttachToComponent` (`self.HitCollision`) (`self.SK_Equipment`) (`self.CollisionSocketName`) "SnapToTarget" "KeepWorld" "KeepWorld" true))

(event `self.HitCollision.OnComponentHit`
  (params (HitComponent :type "PrimitiveComponent Object Reference") (OtherActor :type "Actor Object Reference") (OtherComp :type "PrimitiveComponent Object Reference") (NormalImpulse :type "Vector Structure") (Hit :type "HitResult Structure (by ref)"))
  (bind _returnvalue (`self.GetComponentByClass` OtherActor "/Game/Blueprint/Destructible/BPC_Destructible.BPC_Destructible_C"))
  (bind _isnewitem (`self.HitActorValidation` OtherActor))
  (if _isnewitem
    (`/Engine/EditorBlueprintResources/StandardMacros.IsValid` _returnvalue
      (:`Is Valid`
        (`/Game/Blueprint/Destructible/BPC_Destructible.Hit recieved` _returnvalue)))))

(fn `HitActorValidation`
  (params (`Hit Actor` :type "Actor Object Reference") (`Hit Actor Component` :type "ActorComponent Object Reference"))
  (returns (IsNewItem :type Boolean))
  (locals (CurrentIndex :type Integer :default 0))
  (bind _hittedactors (`self.HittedActors`))
  (set `local.CurrentIndex` (`KismetArrayLibrary.Array_LastIndex` _hittedactors))
  (bind _returnvalue (`KismetArrayLibrary.Array_AddUnique` _hittedactors `Hit Actor`))
  (return (> _returnvalue (`local.CurrentIndex`))))

(fn `UserConstructionScript`
  (`parent.UserConstructionScript`))