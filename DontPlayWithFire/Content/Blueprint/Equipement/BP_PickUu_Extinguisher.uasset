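; Fire extinguisher pickup that equips the player fireman when picked up.
; Its PickupBehavior event calls AddBPCExtinguisher on the fireman with manual attachment off, clears the fireman's PickupObject reference and destroys the pickup actor.
; All other events and the construction script hold only parent calls, with BeginPlay, overlap and Tick disabled.
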(event `self.PickupBehavior`
  (params (PlayerFireman :type "/Game/ThirdPerson/Blueprints/BP_FireMan Object Reference"))
  (`AddComponent|NODE_AddBPC_Extinguisher-0` :`self` PlayerFireman)
  (set `/Game/ThirdPerson/Blueprints/BP_FireMan.PickupObject` null PlayerFireman)
  (`self.K2_DestroyActor`))

(fn `UserConstructionScript`
  (`parent.UserConstructionScript`))