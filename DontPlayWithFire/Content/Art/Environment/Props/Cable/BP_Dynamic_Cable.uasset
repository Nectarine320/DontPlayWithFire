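; Dynamic cable prop that strings instanced static meshes along a simulated Cable component.
; The construction script spans the cable between the StartP and EndP components and sets its length from their distance times a slack factor.
; Every tick it clears and rebuilds the instances at the cable's particle locations, skipping the first, with no rotation, so the meshes follow the simulation.
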(event `self.ReceiveTick`
  (params (DeltaSeconds :type "Float (single-precision)"))
  (bind _locations (`CableComponent.GetCableParticleLocations` (`self.Cable`)))
  (`InstancedStaticMeshComponent.ClearInstances` (`self.InstancedStaticMesh`))
  (for _index (range 1 (`KismetArrayLibrary.Array_Length` _locations))
    (`InstancedStaticMeshComponent.AddInstance` (`self.InstancedStaticMesh`) (`KismetMathLibrary.MakeTransform` (`|GetArrayItem` _locations _index)) true)))

(fn `UserConstructionScript`
  (bind _cable (`self.Cable`))
  (bind _relativelocation (`SceneComponent.RelativeLocation` (`self.StartP`)))
  (bind _relativelocation_2 (`SceneComponent.RelativeLocation` (`self.EndP`)))
  (`SceneComponent.K2_SetRelativeLocation` _cable _relativelocation false false)
  (set `CableComponent.EndLocation` (- _relativelocation_2 _relativelocation) _cable)
  (set `CableComponent.CableLength` (* (`KismetMathLibrary.Vector_Distance` _relativelocation _relativelocation_2) (`self.Cableslack`)) _cable))